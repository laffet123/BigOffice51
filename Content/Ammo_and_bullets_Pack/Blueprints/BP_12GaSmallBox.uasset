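; Configurable 12 gauge small ammo box prop, built entirely in the Construction Script.
; It toggles and rotates the cap, then gives each instanced ammo mesh a seeded random roll within a set range.
; It removes instances in proportion to CountAmmoIn, either at seeded random indices or from the first index.
; It also applies ammo visibility and shadow casting, plus separate cull distances for ammo and box.
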(fn `UserConstructionScript`
  (bind _ammo_visible (`self.Ammo visible`))
  (`|ExecutionSequence`
    (:`then_0`
      ;[1 1 1] Cap Visible
      (`/Game/Ammo_and_bullets_Pack/Blueprints/Macroses/On-Off_Macro.On/Off Macro` (`self.StaticMeshComponent0`) (`self.Visible Cap`))
      ;[1 1 1] Cap rotation
      (`SceneComponent.K2_AddRelativeRotation` (`self.StaticMeshComponent0`) (`KismetMathLibrary.MakeRotator` 0.0 (`self.Rotation Cap`)) false false))
    (:`then_1`
      ;[1 1 1] Set up seed for random seed
      (set `self.Count ammo seed` (`KismetMathLibrary.MakeRandomStream` (`self.= Count ammo Seed =`)))
      (set `self.Rotation ammo Seed` (`KismetMathLibrary.MakeRandomStream` (`self.= Rotation Ammo Seed =`))))
    (:`then_2`
      ;[1 1 1] Update Ammo Transform
      (for _index (range (+ (`InstancedStaticMeshComponent.GetInstanceCount` (`self.InstancedStaticMesh`)) 1))
        (bind _outinstancetransform (`InstancedStaticMeshComponent.GetInstanceTransform` (`self.InstancedStaticMesh`) _index false))
        (`InstancedStaticMeshComponent.UpdateInstanceTransform` (`self.InstancedStaticMesh`) _index (`KismetMathLibrary.MakeTransform` (`KismetMathLibrary.MakeVector` (.x (.location _outinstancetransform)) (.y (.location _outinstancetransform)) (.z (.location _outinstancetransform))) (`KismetMathLibrary.MakeRotator` (`KismetMathLibrary.RandomFloatInRangeFromStream` (`self.Min ammo Rotation`) (`self.Max ammo Rotation`) (`self.Rotation ammo Seed`)) (.pitch (.rotation _outinstancetransform)) (.yaw (.rotation _outinstancetransform)))) false false false)))
    (:`then_3`
      ;[1 1 1] Amount of remote ammo
      (if (`self.Use random count of ammo`)
        (for _ (range (+ (`KismetMathLibrary.FTrunc` (* (`self.Count ammo in %`) 0.08)) 1))
          (`InstancedStaticMeshComponent.RemoveInstance` (`self.InstancedStaticMesh`) (`KismetMathLibrary.RandomIntegerInRangeFromStream` 0 (`InstancedStaticMeshComponent.GetInstanceCount` (`self.InstancedStaticMesh`)) (`self.Count ammo seed`))))
        (else
          (for _ (range (`KismetMathLibrary.FTrunc` (`KismetMathLibrary.Abs` (* (`self.Count ammo in %`) 0.08))))
            (`InstancedStaticMeshComponent.RemoveInstance` (`self.InstancedStaticMesh`) 0)))))
    (:`then_4`
      ;[1 1 1] Ammo Visible
      (`SceneComponent.SetVisibility` (`self.InstancedStaticMesh`) _ammo_visible false)
      (`PrimitiveComponent.SetCastShadow` (`self.InstancedStaticMesh`) _ammo_visible))
    (:`then_5`
      ;[1 1 1] Draw Distance
      (`PrimitiveComponent.SetCullDistance` (`self.InstancedStaticMesh`) (`self.Ammo Draw Distance (0 - Infinity)`))
      (`PrimitiveComponent.SetCullDistance` (`self.StaticMeshComponent01`) (`self.Box Draw Distance (0 - Infinity)`))
      (`PrimitiveComponent.SetCullDistance` (`self.StaticMeshComponent0`) (`self.Box Draw Distance (0 - Infinity)`)))))