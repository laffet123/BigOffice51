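; BP_5-56GaMidBox is a configurable 5.56 ammo box prop with a cap and visible rounds, built entirely in the Construction Script.
; It fills the box with two staggered, opposite-facing rows of rounds through one InstancedStaticMesh to keep them cheap.
; Exposed variables set cap visibility and pitch, ammo visibility with shadows, one of two box materials, and separate cull distances for box and ammo.
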(fn `UserConstructionScript`
  (bind _ammo_visible (`self.Ammo visible`))
  (`|ExecutionSequence`
    (:`then_0`
      ;[1 1 1] Cap Visible
      (`/Game/Ammo_and_bullets_Pack/Blueprints/Macroses/On-Off_Macro.On/Off Macro` (`self.StaticMeshComponent0`) (`self.Visible Cap`))
      ;[1 1 1] Cap rotation
      (`SceneComponent.K2_AddRelativeRotation` (`self.StaticMeshComponent0`) (`KismetMathLibrary.MakeRotator` 0.0 (`self.Rotation Cap`)) false false))
    (:`then_1`
      ;[1 1 1] First row
      (for _index (range 25)
        (`InstancedStaticMeshComponent.AddInstance` (`self.InstancedStaticMesh`) (`KismetMathLibrary.MakeTransform` (`KismetMathLibrary.MakeVector` 0.0 (* _index (`self.Space`))) (struct) (1.0 1.0 1.0)) false)))
    (:`then_2`
      ;[1 1 1] Second row
      (for _index_2 (range 24)
        (`InstancedStaticMeshComponent.AddInstance` (`self.InstancedStaticMesh`) (`KismetMathLibrary.MakeTransform` (`KismetMathLibrary.MakeVector` 10.0 (+ (* _index_2 (`self.Space`)) 0.5)) (struct :`Yaw` 180.0)) false)))
    (:`then_3`
      ;[1 1 1] Ammo Visible
      (`SceneComponent.SetVisibility` (`self.InstancedStaticMesh`) _ammo_visible false)
      (`PrimitiveComponent.SetCastShadow` (`self.InstancedStaticMesh`) _ammo_visible))
    (:`then_4`
      ;[1 1 1] Material variant
      (switch `int` (`self.Material variant`)
        (:`1`
          (`PrimitiveComponent.SetMaterial` (`self.StaticMeshComponent0`) 0 "/Game/Ammo_and_bullets_Pack/Materials/Instances/MI_5-56GaMidBoxV2.MI_5-56GaMidBoxV2")
          (`PrimitiveComponent.SetMaterial` (`self.StaticMeshComponent01`) 0 "/Game/Ammo_and_bullets_Pack/Materials/Instances/MI_5-56GaMidBoxV2.MI_5-56GaMidBoxV2"))
        (:`2`
          (`PrimitiveComponent.SetMaterial` (`self.StaticMeshComponent0`) 0 "/Game/Ammo_and_bullets_Pack/Materials/Instances/MI_5-56GaMidBox.MI_5-56GaMidBox")
          (`PrimitiveComponent.SetMaterial` (`self.StaticMeshComponent01`) 0 "/Game/Ammo_and_bullets_Pack/Materials/Instances/MI_5-56GaMidBox.MI_5-56GaMidBox"))))
    (:`then_5`
      ;[1 1 1] Draw Distance
      (`PrimitiveComponent.SetCullDistance` (`self.InstancedStaticMesh`) (`self.Ammo Draw Distance (0 - Infinity)`))
      (`PrimitiveComponent.SetCullDistance` (`self.StaticMeshComponent01`) (`self.Box Draw Distance (0 - Infinity)`))
      (`PrimitiveComponent.SetCullDistance` (`self.StaticMeshComponent0`) (`self.Box Draw Distance (0 - Infinity)`)))))