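; Strobe light prop Blueprint from the Favela megapack that animates a material on its static mesh.
; On BeginPlay it creates a dynamic material instance for the mesh's second material slot.
; Each Tick it accumulates time scaled by a Multiply speed factor, samples the Light float curve at that time and writes the result to the material's Time parameter.
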(event `self.ReceiveBeginPlay`
  (bind _returnvalue (`PrimitiveComponent.CreateDynamicMaterialInstance` (`self.StaticMesh`) 1 (`self.Material`) "None"))
  (set `self.Mat` _returnvalue))

(event `self.ReceiveTick`
  (params (DeltaSeconds :type "Float (single-precision)"))
  (set `self.Time` (+ (`self.Time`) (* DeltaSeconds (`self.Multiply`))))
  (`MaterialInstanceDynamic.SetScalarParameterValue` (`self.Mat`) "Time" (`CurveFloat.GetFloatValue` (`self.Light`) (`self.Time`))))

(fn `UserConstructionScript`)