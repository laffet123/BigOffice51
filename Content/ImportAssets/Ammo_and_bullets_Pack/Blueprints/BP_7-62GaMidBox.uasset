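; Prop Blueprint for a mid-size 7.62 ammo box, assembled entirely in the Construction Script with no active gameplay logic.
; Exposed variables set the cap's visibility and rotation, the ammo's visibility and shadow, and separate cull distances for ammo and box.
; The rounds are instanced static meshes laid out by loops in two offset, opposite-facing rows at a configurable spacing.
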(fn `UserConstructionScript`
  (bind _ammo_visible (`self.Ammo visible`))
  (`|ExecutionSequence`
    (:`then_0`
      ;[1 1 1] Cap Visible
      (`/Game/ImportAssets/Ammo_and_bullets_Pack/Blueprints/Macroses/On-Off_Macro.On/Off Macro` (`self.StaticMeshComponent0`) (`self.Visible Cap`))
      ;[1 1 1] Cap rotation
      (`SceneComponent.K2_AddRelativeRotation` (`self.StaticMeshComponent0`) (`KismetMathLibrary.MakeRotator` 0.0 (`self.Rotation Cap`)) false false))
    (:`then_1`
      ;[1 1 1] First row
      (for _index (range 24)
        (`InstancedStaticMeshComponent.AddInstance` (`self.InstancedStaticMesh`) (`KismetMathLibrary.MakeTransform` (`KismetMathLibrary.MakeVector` (* _index (`self.Space`))) (struct :`Yaw` -90.0)) false)))
    (:`then_2`
      ;[1 1 1] Second row
      (for _index_2 (range 23)
        (`InstancedStaticMeshComponent.AddInstance` (`self.InstancedStaticMesh`) (`KismetMathLibrary.MakeTransform` (`KismetMathLibrary.MakeVector` (+ (* _index_2 (`self.Space`)) 0.5) -8.0 -1.1) (struct :`Yaw` 90.0)) false)))
    (:`then_3`
      ;[1 1 1] Ammo Visible
      (`SceneComponent.SetVisibility` (`self.InstancedStaticMesh`) _ammo_visible false)
      (`PrimitiveComponent.SetCastShadow` (`self.InstancedStaticMesh`) _ammo_visible))
    (:`then_4`
      ;[1 1 1] Draw Distance
      (`PrimitiveComponent.SetCullDistance` (`self.InstancedStaticMesh`) (`self.Ammo Draw Distance (0 - Infinity)`))
      (`PrimitiveComponent.SetCullDistance` (`self.StaticMeshComponent01`) (`self.Box Draw Distance (0 - Infinity)`))
      (`PrimitiveComponent.SetCullDistance` (`self.StaticMeshComponent0`) (`self.Box Draw Distance (0 - Infinity)`)))))