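; BP_CharRoot is a character base Blueprint that plays surface-dependent footstep sounds.
; PlaySoundFootR and PlaySoundFootL call GetSoundQueFromRay, which traces down from that foot, or the Mesh if none, and picks a cue by physical surface type.
; The sound plays at the Mesh location, not at the foot.
; GetRFoot, GetLFoot and GetCam are empty stubs, apparently for child classes to override.
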(event `/Game/_Game/MyNew/PJH/BP/Interface/BP_IF_Char.PlaySound_FootR`
  (bind _output_sound (`self.GetSoundQue_FromRay` true))
  (`/Engine/EditorBlueprintResources/StandardMacros.IsValid` _output_sound
    (:`Is Valid`
      (`GameplayStatics.PlaySoundAtLocation` _output_sound (`SceneComponent.K2_GetComponentLocation` (`self.Mesh`)) (struct) 1.0 1.0 0.0 null null null null))))

(event `/Game/_Game/MyNew/PJH/BP/Interface/BP_IF_Char.PlaySound_FootL`
  (bind _output_sound (`self.GetSoundQue_FromRay` false))
  (`/Engine/EditorBlueprintResources/StandardMacros.IsValid` _output_sound
    (:`Is Valid`
      (`GameplayStatics.PlaySoundAtLocation` _output_sound (`SceneComponent.K2_GetComponentLocation` (`self.Mesh`)) (struct) 1.0 1.0 0.0 null null null null))))

(fn `GetCam`
  (returns (Camera :type "SceneComponent Object Reference"))
  (return null))

(fn `GetLFoot`
  (returns (ArrowComp :type "ArrowComponent Object Reference"))
  (return null))

(fn `GetRFoot`
  (returns (ArrowComp :type "ArrowComponent Object Reference"))
  (return null))

(fn `GetSoundQue_FromRay`
  (params (IsR :type Boolean))
  (returns (Output_Sound :type "SoundCue Object Reference"))
  (bind _returnvalue (select `bool` IsR :`false` (`self.GetLFoot`) :`true` (`self.GetRFoot`) :!type "SceneComponent Object Reference"))
  (bind _returnvalue_2 (`SceneComponent.K2_GetComponentLocation` (select `bool` (`KismetSystemLibrary.IsValid` _returnvalue) :`false` (`self.Mesh`) :`true` _returnvalue :!type "SceneComponent Object Reference")))
  (bind (_outhit _returnvalue_3) (`KismetSystemLibrary.LineTraceSingle` _returnvalue_2 (- _returnvalue_2 (0.0 0.0 80.0)) "TraceTypeQuery1"))
  (if _returnvalue_3
    (return (select `byte` (`GameplayStatics.GetSurfaceType` _outhit) :`0` "/Game/_Game/MyNew/Sound/foot_R_Cue.foot_R_Cue" :`1` "/Game/_Game/MyNew/Sound/FootStep/Grass/Footsteps_Walk_Grass_Mono_01_Cue.Footsteps_Walk_Grass_Mono_01_Cue" :`2` "/Game/_Game/MyNew/Sound/foot_R_Cue.foot_R_Cue" :`3` "/Game/_Game/MyNew/Sound/FootStep/Metal/Footsteps_MetalV2_Walk_01_Cue.Footsteps_MetalV2_Walk_01_Cue" :`4` "/Game/_Game/MyNew/Sound/FootStep/Dirty/Wood/Footsteps_Wood_Walk_10_Cue.Footsteps_Wood_Walk_10_Cue" :`5` "/Game/_Game/MyNew/Sound/FootStep/Sand/Footsteps_Sand_Walk_04_Cue.Footsteps_Sand_Walk_04_Cue" :`6` "/Game/_Game/MyNew/Sound/FootStep/Dirty/Footsteps_DirtyGround_Walk_10_Cue.Footsteps_DirtyGround_Walk_10_Cue" :!type "SoundCue Object Reference"))
    (else
      (return null))))

(fn `UserConstructionScript`)