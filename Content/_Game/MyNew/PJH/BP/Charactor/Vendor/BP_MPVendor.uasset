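; Multiplayer vendor NPC that players interact with to open a shop, using a Jig multiplayer inventory component.
; On interaction it opens a shop paired with the base stash when in base camp, adds the vendor widget if not already visible, and flags VendorOn.
; A looping timer notifies the player once they stray too far from where they interacted.
; It also shows an interact prompt, greets overlapping players with a montage, and spawns dropped items nearby.
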(event `/Game/_Game/JigSInventory/Jigsaw/Components/Interfaces/BP_MpInteractInterface.OnEndInteract`
  (`SceneComponent.SetVisibility` (`self.Widget`) false false))

(event `/Game/_Game/JigSInventory/Jigsaw/Components/Interfaces/BP_MpInteractInterface.OnBeginInteract`
  (params (InteractingActor :type "Actor Object Reference") (Options :type "Array of /Game/_Game/JigSInventory/Jigsaw/Components/Interfaces/E_InteractOptions Enum (by ref)" :default _))
  (`|ExecutionSequence`
    (:`then_0`
      (bind _asbp_interact_widget (cast `/Game/_Game/JigSInventory/Jigsaw/Widgets/BP_InteractWidget` (`WidgetComponent.GetUserWidgetObject` (`self.Widget`))))
      (`/Game/_Game/JigSInventory/Jigsaw/Widgets/BP_InteractWidget.SetName` _asbp_interact_widget "Interact" (`self.Vendor`)))
    (:`then_1`
      (`SceneComponent.SetVisibility` (`self.Widget`) true false))))

(event `/Game/_Game/JigSInventory/Jigsaw/Components/Interfaces/BP_MpInteractInterface.OnExecuteInteract`
  (params (InteractingActor :type "Actor Object Reference") (Option :type "/Game/_Game/JigSInventory/Jigsaw/Components/Interfaces/E_InteractOptions Enum" :default "NewEnumerator0"))
  (`|ExecutionSequence`
    (:`then_0`
      (`self.LCreateVendorInBasecamp` InteractingActor)
      (set `/Game/_Game/MyNew/PJH/BP_GameInstance.VendorOn?` true (`self.CastedGameInstance`)))
    (:`then_1`
      (set `self.CurrentActor` InteractingActor)
      (if (not (`/Game/_Game/JigSInventory/Jigsaw/Components/BP_Multiplayer.IsInventoryVisible?` (`self.BP_JigMultiplayer`)))
        (bind _inventorywidgetref (`/Game/_Game/JigSInventory/Jigsaw/Components/BP_Multiplayer.SetupInventoryWidget` (`self.BP_JigMultiplayer`) true false))
        (message `/Game/_Game/JigSInventory/Jigsaw/Components/Interfaces/BP_JigCharacterInterface.AddJigWidgetToContent` InteractingActor _inventorywidgetref (`self.Vendor`))
        (message `/Game/_Game/JigSInventory/Jigsaw/Components/Interfaces/BP_JigCharacterInterface.RequestServerData` InteractingActor (`self.BP_JigMultiplayer`))
        (set `self.InteractingActorLoc` (`self.K2_GetActorLocation` InteractingActor))
        (`KismetSystemLibrary.K2_SetTimer` null "CheckDistanceFromActor" 0.1 true)))))

(event `/Game/_Game/JigSInventory/Jigsaw/Components/Interfaces/BP_MpInteractInterface.OnServerExecuteInteract`)

(event `/Game/_Game/JigSInventory/Jigsaw/Components/Interfaces/BP_MpInteractInterface.OnExecuteInteractEnded`
  (set `/Game/_Game/MyNew/PJH/BP_GameInstance.VendorOn?` false (`self.CastedGameInstance`))
  (set `self.CurrentActor` null)
  (`KismetSystemLibrary.K2_SetTimer` null "CheckDistanceFromActor" 0.1 true))

(event `self.Sphere1.OnComponentBeginOverlap`
  (params (OverlappedComponent :type "PrimitiveComponent Object Reference") (OtherActor :type "Actor Object Reference") (OtherComp :type "PrimitiveComponent Object Reference") (OtherBodyIndex :type Integer) (bFromSweep :type Boolean) (SweepResult :type "HitResult Structure (by ref)"))
  (cast `/Game/_Game/MyNew/PJH/BP/Charactor/Player/BP_MainChar` OtherActor)
  (`|PlayMontage` (`self.SkeletalMesh`) "/Game/_Game/MyNew/PJH/BP/Charactor/Vendor/Anim/Standing_Greeting__1__Montage1.Standing_Greeting__1__Montage1"))

(fn `CanInteract`
  (returns (Result :type Boolean))
  (return true))

(fn `CastedGameInstance`
  (returns (`BP Game Instance` :type "/Game/_Game/MyNew/PJH/BP_GameInstance Object Reference"))
  (return (cast `/Game/_Game/MyNew/PJH/BP_GameInstance` (`GameplayStatics.GetGameInstance`) :!pure true)))

(fn `CheckDistanceFromActor`
  (bind _currentactor (`self.CurrentActor`))
  ;[0.151 0.151 0.151] close the vendor widget if the player is too far
  (`/Engine/EditorBlueprintResources/StandardMacros.IsValid` _currentactor
    (:`Is Valid`
      (if (> (`KismetMathLibrary.VSize` (- (`self.InteractingActorLoc`) (`self.K2_GetActorLocation` _currentactor))) 300.0)
        (`KismetSystemLibrary.K2_ClearTimer` null "CheckDistanceFromActor")
        (message `/Game/_Game/JigSInventory/Jigsaw/Components/Interfaces/BP_JigCharacterInterface.OnInteractActorOverDistance` (`self.CurrentActor`) self)
        (set `self.CurrentActor` null)))
    (:`Is Not Valid`
      (`KismetSystemLibrary.K2_ClearTimer` null "CheckDistanceFromActor"))))

(fn `GetItemInfo`
  (returns (Info :type "/Game/_Game/JigSInventory/Jigsaw/Data/DataAsset/DA_Item Object Reference") (Count :type Integer) (RandomStatsConfig :type "/Game/_Game/JigSInventory/Jigsaw/Data/ST_RandomStatsConfig Structure"))
  (return null 0))

(fn `GetMultiplayerComponent`
  (returns (JigComp :type "/Game/_Game/JigSInventory/Jigsaw/Components/BP_Multiplayer Object Reference"))
  (return (`self.BP_JigMultiplayer`)))

(fn `JigMP_GetLootWidget`
  (returns (Result :type "Widget Object Reference") (`Valid?` :type Boolean))
  (return null false))

(fn `JigMP_OnContainersSwap`
  (params (Container1 :type "/Game/_Game/JigSInventory/Jigsaw/Widgets/WBP_Container Object Reference") (Container2 :type "/Game/_Game/JigSInventory/Jigsaw/Widgets/WBP_Container Object Reference"))
  (returns (Result :type Boolean))
  (return false))

(fn `JigMP_OnItemAdded`
  (params (ItemUID :type "Guid Structure") (FromContainerUID :type "Guid Structure") (ToContainerUID :type "Guid Structure") (FromComponent :type "/Game/_Game/JigSInventory/Jigsaw/Components/BP_Multiplayer Object Reference"))
  (returns (Result :type Boolean))
  (return false))

(fn `JigMP_OnItemConsumed`
  (params (ConsumedItem :type "/Game/_Game/JigSInventory/Jigsaw/Data/ST_RepItemInfo Structure") (Amount :type Integer) (Remaining :type Integer) (InsideOf :type "/Game/_Game/JigSInventory/Jigsaw/Data/ST_RepItemInfo Structure") (FromContainer :type Name) (CustomData :type String))
  (returns (Result :type Boolean))
  (return false))

(fn `JigMP_OnItemDropped`
  (params (ItemUID :type "Guid Structure") (FromContainerUID :type "Guid Structure") (ActorRef :type "Actor Object Reference"))
  (returns (Result :type Boolean))
  (return false))

(fn `JigMP_OnItemMoved`
  (params (ItemUID :type "Guid Structure") (FromContainerUID :type "Guid Structure") (ToContainerUID :type "Guid Structure"))
  (returns (Result :type Boolean))
  (return false))

(fn `JigMP_OnItemRemoved`
  (params (ItemUID :type "Guid Structure") (FromContainerUID :type "Guid Structure") (ToContainerUID :type "Guid Structure") (ToComponent :type "/Game/_Game/JigSInventory/Jigsaw/Components/BP_Multiplayer Object Reference"))
  (returns (Result :type Boolean))
  (return false))

(fn `JigMP_OnMainContainerItemAdded`
  (params (ToContainerUID :type "Guid Structure") (ItemUID :type "Guid Structure") (ToContainerName :type Name) (ItemInfo :type "/Game/_Game/JigSInventory/Jigsaw/Data/ST_RepItemInfo Structure") (FromMain :type Name))
  (returns (Result :type Boolean) (ActorRef :type "Actor Object Reference"))
  (return false null))

(fn `JigMP_OnMainContainerItemRemoved`
  (params (FromContainerUID :type "Guid Structure") (ItemUID :type "Guid Structure") (ContainerName :type Name) (ItemRemovedInfo :type "/Game/_Game/JigSInventory/Jigsaw/Data/ST_RepItemInfo Structure"))
  (returns (Result :type Boolean))
  (return false))

(fn `JigMP_OnPickupAdded`
  (params (Info :type "/Game/_Game/JigSInventory/Jigsaw/Data/ST_RepItemInfo Structure") (ItemUID :type "Guid Structure") (ToContainerUID :type "Guid Structure") (ToContainer :type Name))
  (returns (Result :type Boolean))
  (return false))

(fn `JigMP_OnPickupEquipped`
  (params (ActorRef :type "Actor Object Reference") (ToContainerName :type Name) (UID :type "Guid Structure") (ToContainerUID :type "Guid Structure") (Info :type "/Game/_Game/JigSInventory/Jigsaw/Data/ST_RepItemInfo Structure"))
  (returns (Result :type Boolean))
  (return false))

(fn `JigMP_OnRequestDropItem`
  (params (ItemInfo :type "/Game/_Game/JigSInventory/Jigsaw/Data/ST_RepItemInfo Structure") (ContainerName :type Name) (FromJSI :type "/Game/_Game/JigSInventory/Jigsaw/Widgets/WBP_Container Object Reference"))
  (returns (ActorRef :type "Actor Object Reference"))
  (`|ExecutionSequence`
    (:`then_0`
      (bind _returnvalue (`|SpawnActorFromClass` (`/Game/_Game/JigSInventory/Jigsaw/Data/DataAsset/DA_Item.ActorClass` (`.ItemID_28_01CA27D84AF7D1014D9E2E83894C1848` (break `/Game/_Game/JigSInventory/Jigsaw/Data/ST_RepItemInfo` ItemInfo))) (`KismetMathLibrary.MakeTransform` (+ (`self.K2_GetActorLocation`) (* (`self.GetActorForwardVector`) 200.0) (`KismetMathLibrary.MakeVector` (`KismetMathLibrary.RandomFloatInRange` -75.0 75.0) (`KismetMathLibrary.RandomFloatInRange` -75.0 75.0))) (`KismetMathLibrary.MakeRotator` 0.0 0.0 (`KismetMathLibrary.RandomFloatInRange` -180.0 180.0))) "AdjustIfPossibleButAlwaysSpawn" "OverrideRootScale" null null))
      (return _returnvalue))
    (:`then_1`
      (return null))))

(fn `JigMP_OnTwoContainersSwap`
  (params (FromContainer :type Name) (ToContainer :type Name))
  (returns (Result :type Boolean))
  (return false))

(fn `JigMP_OnUpdateChamberUID`
  (params (NewUID :type "Guid Structure"))
  (returns (Result :type Boolean))
  (return false))

(fn `LCreateVendorInBasecamp`
  (params (interacingActor :type "Actor Object Reference"))
  (bind _bp_jigmultiplayer (`self.BP_JigMultiplayer`))
  (bind _asbp_mpgame_mode (cast `/Game/_Game/JigSInventory/Demo/BP_MPGameMode` (`GameplayStatics.GetGameMode`) :!pure true))
  (if (`/Game/_Game/JigSInventory/Demo/BP_MPGameMode.IsBaseCamp` _asbp_mpgame_mode)
    (bind _jigcomp (message `/Game/_Game/JigSInventory/Jigsaw/Components/Interfaces/BP_MpInteractInterface.GetMultiplayerComponent` (`/Game/_Game/JigSInventory/Demo/BP_MPGameMode.BaseStash` _asbp_mpgame_mode)))
    (bind _inventorywidgetref (`/Game/_Game/JigSInventory/Jigsaw/Components/BP_Multiplayer.SetupInventoryWidget` _jigcomp false false)) ; Stash Widget 생성
    (bind _inventorywidgetref_2 (`/Game/_Game/JigSInventory/Jigsaw/Components/BP_Multiplayer.SetupInventoryWidget` _bp_jigmultiplayer true false)) ; Vendor 위젯 생성
    (message `/Game/_Game/JigSInventory/Jigsaw/Components/Interfaces/BP_JigCharacterInterface.LOnShopRequest` interacingActor _inventorywidgetref _inventorywidgetref_2 _bp_jigmultiplayer)
    (message `/Game/_Game/JigSInventory/Jigsaw/Components/Interfaces/BP_JigCharacterInterface.RequestServerData` interacingActor _jigcomp)
    (message `/Game/_Game/JigSInventory/Jigsaw/Components/Interfaces/BP_JigCharacterInterface.RequestServerData` interacingActor (`self.BP_JigMultiplayer`))
    (set `self.InteractingActorLoc` (`self.K2_GetActorLocation` interacingActor))
    (`KismetSystemLibrary.K2_SetTimer` null "CheckDistanceFromActor" 0.1 true)))

(fn `SetCanInteract`
  (params (CanInteract :type Boolean) (EnablePhysics :type Boolean))
  (returns (Result :type Boolean))
  (return false))

(fn `SetPickupCount`
  (params (NewCount :type Integer))
  (returns (Result :type Boolean))
  (return false))

(fn `UserConstructionScript`)