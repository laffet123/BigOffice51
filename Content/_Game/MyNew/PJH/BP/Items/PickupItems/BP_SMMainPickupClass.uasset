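; Base static-mesh item pickup that plugs into the interaction system and the Jig multiplayer inventory.
; Interaction, item info, count and interactability are forwarded to BPPickupComponent, while a widget shows the pickup name and options.
; Jig item add, move, drop and remove callbacks refresh attachments; most other callbacks are stubbed to false.
; Drop requests spawn the item's actor class nearby with random offset and yaw.
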(event `/Game/_Game/JigSInventory/Jigsaw/Components/Interfaces/BP_MpInteractInterface.OnExecuteInteract`
  (params (InteractingActor :type "Actor Object Reference") (Option :type "/Game/_Game/JigSInventory/Jigsaw/Components/Interfaces/E_InteractOptions Enum" :default "NewEnumerator0"))
  ;[0.06771 0.06771 0.06771] Interaction
  (`/Game/_Game/JigSInventory/Jigsaw/Pickup/BP_PickupComponent.OnExecuteInteract` (`self.BP_PickupComponent`) InteractingActor Option))

(event `/Game/_Game/JigSInventory/Jigsaw/Components/Interfaces/BP_MpInteractInterface.OnBeginInteract`
  (params (InteractingActor :type "Actor Object Reference") (Options :type "Array of /Game/_Game/JigSInventory/Jigsaw/Components/Interfaces/E_InteractOptions Enum (by ref)" :default _))
  ;[0.06771 0.06771 0.06771] Interaction
  (`|ExecutionSequence`
    (:`then_0`
      (bind _asbp_interact_widget (cast `/Game/_Game/JigSInventory/Jigsaw/Widgets/BP_InteractWidget` (`WidgetComponent.GetUserWidgetObject` (`self.Widget`))))
      (`/Game/_Game/JigSInventory/Jigsaw/Widgets/BP_InteractWidget.SetName` _asbp_interact_widget "Pickup" (`/Game/_Game/JigSInventory/Jigsaw/Pickup/BP_PickupComponent.GetPickupName` (`self.BP_PickupComponent`)))
      (`/Game/_Game/JigSInventory/Jigsaw/Widgets/BP_InteractWidget.InitOptions` _asbp_interact_widget Options))
    (:`then_1`
      (`SceneComponent.SetVisibility` (`self.Widget`) true false))))

(event `/Game/_Game/JigSInventory/Jigsaw/Components/Interfaces/BP_MpInteractInterface.OnEndInteract`
  ;[0.06771 0.06771 0.06771] Interaction
  (`SceneComponent.SetVisibility` (`self.Widget`) false false))

(event `/Game/_Game/JigSInventory/Jigsaw/Components/Interfaces/BP_MpInteractInterface.SetInteractOption`
  (params (Option :type "/Game/_Game/JigSInventory/Jigsaw/Components/Interfaces/E_InteractOptions Enum" :default "NewEnumerator0"))
  ;[0.06771 0.06771 0.06771] Interaction
  (bind _asbp_interact_widget (cast `/Game/_Game/JigSInventory/Jigsaw/Widgets/BP_InteractWidget` (`WidgetComponent.GetUserWidgetObject` (`self.Widget`))))
  (`/Game/_Game/JigSInventory/Jigsaw/Widgets/BP_InteractWidget.SetOption` _asbp_interact_widget (select `/Game/_Game/JigSInventory/Jigsaw/Components/Interfaces/E_InteractOptions` Option :`NewEnumerator1` 1)))

(fn `CanInteract`
  (returns (Result :type Boolean))
  ;[0.151 0.151 0.151] See if we can interact
  (return (`/Game/_Game/JigSInventory/Jigsaw/Pickup/BP_PickupComponent.CanInteract?` (`self.BP_PickupComponent`))))

(fn `GetItemInfo`
  (returns (Info :type "/Game/_Game/JigSInventory/Jigsaw/Data/DataAsset/JigsawItem_DataAsset Object Reference") (Count :type Integer) (RandomStatsConfig :type "/Game/_Game/JigSInventory/Jigsaw/Data/S_RandomStatsConfig Structure"))
  (bind _bp_pickupcomponent (`self.BP_PickupComponent`))
  ;[0.151 0.151 0.151] Return the pickup info from data table
  (return (`/Game/_Game/JigSInventory/Jigsaw/Pickup/BP_PickupComponent.ItemDataAsset` _bp_pickupcomponent) (`/Game/_Game/JigSInventory/Jigsaw/Pickup/BP_PickupComponent.GetCount` _bp_pickupcomponent) (`/Game/_Game/JigSInventory/Jigsaw/Pickup/BP_PickupComponent.RandomStatConfig` _bp_pickupcomponent)))

(fn `GetMultiplayerComponent`
  (returns (JigComp :type "/Game/_Game/JigSInventory/Jigsaw/Components/BP_Multiplayer Object Reference"))
  ;[0.151 0.151 0.151] Return Jig multiplayer component
  (return (`self.BP_Multiplayer`)))

(fn `JigMP_GetLootWidget`
  (returns (Result :type "Widget Object Reference") (`Valid?` :type Boolean))
  (return null false))

(fn `JigMP_OnContainersSwap`
  (params (Container1 :type "/Game/_Game/JigSInventory/Jigsaw/Widgets/WBP_Container Object Reference") (Container2 :type "/Game/_Game/JigSInventory/Jigsaw/Widgets/WBP_Container Object Reference"))
  (returns (Result :type Boolean))
  (return false))

(fn `JigMP_OnItemAdded`
  (params (ItemUID :type "Guid Structure") (FromContainerUID :type "Guid Structure") (ToContainerUID :type "Guid Structure") (FromComponent :type "/Game/_Game/JigSInventory/Jigsaw/Components/BP_Multiplayer Object Reference"))
  (returns (Result :type Boolean))
  (`/Game/_Game/JigSInventory/Jigsaw/Pickup/BP_PickupComponent.UpdateAttachments` (`self.BP_PickupComponent`))
  (return true))

(fn `JigMP_OnItemConsumed`
  (params (ConsumedItem :type "/Game/_Game/JigSInventory/Jigsaw/Data/RepItemInfo Structure") (Amount :type Integer) (Remaining :type Integer) (InsideOf :type "/Game/_Game/JigSInventory/Jigsaw/Data/RepItemInfo Structure") (FromContainer :type Name) (CustomData :type String))
  (returns (Result :type Boolean))
  (return false))

(fn `JigMP_OnItemDropped`
  (params (ItemUID :type "Guid Structure") (FromContainerUID :type "Guid Structure") (ActorRef :type "Actor Object Reference"))
  (returns (Result :type Boolean))
  (`/Game/_Game/JigSInventory/Jigsaw/Pickup/BP_PickupComponent.UpdateAttachments` (`self.BP_PickupComponent`))
  (return true))

(fn `JigMP_OnItemMoved`
  (params (ItemUID :type "Guid Structure") (FromContainerUID :type "Guid Structure") (ToContainerUID :type "Guid Structure"))
  (returns (Result :type Boolean))
  (`/Game/_Game/JigSInventory/Jigsaw/Pickup/BP_PickupComponent.UpdateAttachments` (`self.BP_PickupComponent`))
  (return true))

(fn `JigMP_OnItemRemoved`
  (params (ItemUID :type "Guid Structure") (FromContainerUID :type "Guid Structure") (ToContainerUID :type "Guid Structure") (ToComponent :type "/Game/_Game/JigSInventory/Jigsaw/Components/BP_Multiplayer Object Reference"))
  (returns (Result :type Boolean))
  (`/Game/_Game/JigSInventory/Jigsaw/Pickup/BP_PickupComponent.UpdateAttachments` (`self.BP_PickupComponent`))
  (return true))

(fn `JigMP_OnMainContainerItemAdded`
  (params (ToContainerUID :type "Guid Structure") (ItemUID :type "Guid Structure") (ToContainerName :type Name) (ItemInfo :type "/Game/_Game/JigSInventory/Jigsaw/Data/RepItemInfo Structure") (FromMain :type Name))
  (returns (Result :type Boolean) (ActorRef :type "Actor Object Reference"))
  (return false null))

(fn `JigMP_OnMainContainerItemRemoved`
  (params (FromContainerUID :type "Guid Structure") (ItemUID :type "Guid Structure") (ContainerName :type Name) (ItemRemovedInfo :type "/Game/_Game/JigSInventory/Jigsaw/Data/RepItemInfo Structure"))
  (returns (Result :type Boolean))
  (return false))

(fn `JigMP_OnPickupAdded`
  (params (Info :type "/Game/_Game/JigSInventory/Jigsaw/Data/RepItemInfo Structure") (ItemUID :type "Guid Structure") (ToContainerUID :type "Guid Structure") (ToContainer :type Name))
  (returns (Result :type Boolean))
  (return false))

(fn `JigMP_OnPickupEquipped`
  (params (ActorRef :type "Actor Object Reference") (ToContainerName :type Name) (UID :type "Guid Structure") (ToContainerUID :type "Guid Structure") (Info :type "/Game/_Game/JigSInventory/Jigsaw/Data/RepItemInfo Structure"))
  (returns (Result :type Boolean))
  (return false))

(fn `JigMP_OnRequestDropItem`
  (params (ItemInfo :type "/Game/_Game/JigSInventory/Jigsaw/Data/RepItemInfo Structure") (ContainerName :type Name) (FromJSI :type "/Game/_Game/JigSInventory/Jigsaw/Widgets/WBP_Container Object Reference"))
  (returns (ActorRef :type "Actor Object Reference"))
  ;[0.151 0.151 0.151] Dropping an item from the container spawns it in the world
  (`|ExecutionSequence`
    (:`then_0`
      (bind _returnvalue (`|SpawnActorFromClass` (`/Game/_Game/JigSInventory/Jigsaw/Data/DataAsset/JigsawItem_DataAsset.ActorClass` (`.ItemID_28_01CA27D84AF7D1014D9E2E83894C1848` (break `/Game/_Game/JigSInventory/Jigsaw/Data/RepItemInfo` ItemInfo))) (`KismetMathLibrary.MakeTransform` (+ (`self.K2_GetActorLocation`) (`KismetMathLibrary.MakeVector` (`KismetMathLibrary.RandomFloatInRange` -75.0 75.0) (`KismetMathLibrary.RandomFloatInRange` -75.0 75.0) 25.0)) (`KismetMathLibrary.MakeRotator` 0.0 0.0 (`KismetMathLibrary.RandomFloatInRange` -180.0 180.0))) "AdjustIfPossibleButAlwaysSpawn" "OverrideRootScale" null null))
      (return _returnvalue))
    (:`then_1`
      (return null))))

(fn `JigMP_OnTwoContainersSwap`
  (params (FromContainer :type Name) (ToContainer :type Name))
  (returns (Result :type Boolean))
  (return false))

(fn `JigMP_OnUpdateChamberUID`
  (params (NewUID :type "Guid Structure"))
  (returns (Result :type Boolean))
  (return false))

(fn `SetCanInteract`
  (params (CanInteract :type Boolean) (EnablePhysics :type Boolean))
  (returns (Result :type Boolean))
  ;[0.151 0.151 0.151] When this pickup gets equipped, disable physics and interaction
  (bind _result (`/Game/_Game/JigSInventory/Jigsaw/Pickup/BP_PickupComponent.SetCanInteract` (`self.BP_PickupComponent`) CanInteract EnablePhysics))
  (`PrimitiveComponent.SetCollisionEnabled` (`self.StaticMeshComponent`) (select `bool` CanInteract :`false` "NoCollision" :`true` "QueryAndPhysics" :!type "ECollisionEnabled Enum"))
  (return _result))

(fn `SetPickupCount`
  (params (NewCount :type Integer))
  (returns (Result :type Boolean))
  (`/Game/_Game/JigSInventory/Jigsaw/Pickup/BP_PickupComponent.SetCount` (`self.BP_PickupComponent`) NewCount)
  (return true))

(fn `UserConstructionScript`)