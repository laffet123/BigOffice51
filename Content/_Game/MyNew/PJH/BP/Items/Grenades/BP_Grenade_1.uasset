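; Grenade item that works as an interactable until fired, then becomes a thrown projectile that explodes.
; When spawned with IsFired set, it enables projectile movement, switches the mesh to physics simulation shortly after, and after a fuse delay spawns an explosion emitter and destroys itself.
; The CheckIsFired macro gates the interaction events, passing them to the parent class only for unfired grenades.
; The explosion is visual only, with no damage applied here.
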(event `self.ReceiveBeginPlay`
  (if (`self.IsFired`)
    (set `ProjectileMovementComponent.bSimulationEnabled` true (`self.ProjectileMovement`))
    (`|ExecutionSequence`
      (:`then_0`
        (`KismetSystemLibrary.Delay` 0.2)
        (`PrimitiveComponent.SetSimulatePhysics` (`self.StaticMeshComponent`) true))
      (:`then_1`
        (`KismetSystemLibrary.Delay` 3.0)
        (`GameplayStatics.SpawnEmitterAtLocation` "/Game/Realistic_Starter_VFX_Pack_Vol2/Particles/Explosion/P_Explosion_Big_A.P_Explosion_Big_A" (`self.K2_GetActorLocation`) (struct) (5.0 5.0 5.0))
        (`self.K2_DestroyActor`)))))

(event `/Game/_Game/JigSInventory/Jigsaw/Components/Interfaces/BP_MpInteractInterface.OnExecuteInteract`
  (params (InteractingActor :type "Actor Object Reference") (Option :type "/Game/_Game/JigSInventory/Jigsaw/Components/Interfaces/E_InteractOptions Enum" :default "NewEnumerator0"))
  (`self.CheckIsFired`
    (:`else`
      (`parent.OnExecuteInteract` InteractingActor Option))))

(event `/Game/_Game/JigSInventory/Jigsaw/Components/Interfaces/BP_MpInteractInterface.OnBeginInteract`
  (params (InteractingActor :type "Actor Object Reference") (Options :type "Array of /Game/_Game/JigSInventory/Jigsaw/Components/Interfaces/E_InteractOptions Enum (by ref)" :default _))
  (`self.CheckIsFired`
    (:`else`
      (`parent.OnBeginInteract` InteractingActor Options))))

(event `/Game/_Game/JigSInventory/Jigsaw/Components/Interfaces/BP_MpInteractInterface.OnEndInteract`
  (`self.CheckIsFired`
    (:`else`
      (`parent.OnEndInteract`))))

(event `/Game/_Game/JigSInventory/Jigsaw/Components/Interfaces/BP_MpInteractInterface.OnExecuteInteractEnded`
  (`self.CheckIsFired`
    (:`else`
      (`parent.OnExecuteInteractEnded`))))

(fn `UserConstructionScript`
  (`parent.UserConstructionScript`))