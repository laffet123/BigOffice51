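; BP_StageEnter is an interactable raid entrance that opens a stage selection screen for the player.
; A floating text widget labeled "Enter Raid" starts hidden and shows only while interaction focus is active.
; Executing the interaction creates WBP_SelectStage with a self reference and shows the mouse cursor; ending it removes both.
; It is always interactable, and its item, pickup and multiplayer interface functions are empty stubs.
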(event `self.ReceiveBeginPlay`
  (bind _aswbp_float_text (cast `/Game/_Game/MyNew/PJH/BP/WBP_FloatText` (`WidgetComponent.GetUserWidgetObject` (`self.Widget`))))
  (set `/Game/_Game/MyNew/PJH/BP/WBP_FloatText.Var_Text` "Enter Raid" _aswbp_float_text)
  (`SceneComponent.SetVisibility` (`self.Widget`) false false))

(event `/Game/_Game/JigSInventory/Jigsaw/Components/Interfaces/BP_MpInteractInterface.OnBeginInteract`
  (params (InteractingActor :type "Actor Object Reference") (Options :type "Array of /Game/_Game/JigSInventory/Jigsaw/Components/Interfaces/E_InteractOptions Enum (by ref)" :default _))
  (`SceneComponent.SetVisibility` (`self.Widget`) true false))

(event `/Game/_Game/JigSInventory/Jigsaw/Components/Interfaces/BP_MpInteractInterface.OnEndInteract`
  (`SceneComponent.SetVisibility` (`self.Widget`) false false))

(event `/Game/_Game/JigSInventory/Jigsaw/Components/Interfaces/BP_MpInteractInterface.OnExecuteInteract`
  (params (InteractingActor :type "Actor Object Reference") (Option :type "/Game/_Game/JigSInventory/Jigsaw/Components/Interfaces/E_InteractOptions Enum" :default "NewEnumerator0"))
  (bind _returnvalue (`|CreateWidget` "/Game/_Game/MyNew/PJH/BP/Widget/WBP_SelectStage.WBP_SelectStage_C" null self))
  (bind _output_get (set `self.WBP_SelectRef` _returnvalue))
  (`UserWidget.AddToViewport` _output_get 0)
  (set `PlayerController.bShowMouseCursor` true (`GameplayStatics.GetPlayerController` 0)))

(event `/Game/_Game/JigSInventory/Jigsaw/Components/Interfaces/BP_MpInteractInterface.OnExecuteInteractEnded`
  (`Widget.RemoveFromParent` (`self.WBP_SelectRef`))
  (set `self.WBP_SelectRef` null)
  (set `PlayerController.bShowMouseCursor` false (`GameplayStatics.GetPlayerController` 0)))

(fn `CanInteract`
  (returns (Result :type Boolean))
  (return true))

(fn `GetItemInfo`
  (returns (Info :type "/Game/_Game/JigSInventory/Jigsaw/Data/DataAsset/DA_Item Object Reference") (Count :type Integer) (RandomStatsConfig :type "/Game/_Game/JigSInventory/Jigsaw/Data/ST_RandomStatsConfig Structure"))
  (return null 0))

(fn `GetMultiplayerComponent`
  (returns (JigComp :type "/Game/_Game/JigSInventory/Jigsaw/Components/BP_Multiplayer Object Reference"))
  (return null))

(fn `SetCanInteract`
  (params (CanInteract :type Boolean) (EnablePhysics :type Boolean))
  (returns (Result :type Boolean))
  (return false))

(fn `SetPickupCount`
  (params (NewCount :type Integer))
  (returns (Result :type Boolean))
  (return false))

(fn `UserConstructionScript`)