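; Bullet projectile actor for guns that deals point damage and leaves surface impact effects.
; Construction applies lifespan, speed and gravity to its movement component, and BeginPlay ignores the weapon and sets a ten-second self-destroy.
; Sphere overlaps with player-tagged, dynamic, pawn or mesh components deal damage by ammo type, sparing the shooter, then destroy the bullet.
; World Static hits play metal-impact sound, particles and a normal-offset decal before destroying it.
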(event `self.ReceiveBeginPlay`
  (`PrimitiveComponent.IgnoreActorWhenMoving` (`self.Sphere`) (`self.WeaponOwner`) true)
  (set `self.InitalLoc` (`self.K2_GetActorLocation`))
  (`KismetSystemLibrary.Delay` 10.0)
  (`self.K2_DestroyActor`))

(event `self.Sphere.OnComponentBeginOverlap`
  (params (OverlappedComponent :type "PrimitiveComponent Object Reference") (OtherActor :type "Actor Object Reference") (OtherComp :type "PrimitiveComponent Object Reference") (OtherBodyIndex :type Integer) (bFromSweep :type Boolean) (SweepResult :type "HitResult Structure (by ref)"))
  (bind (_bblockinghit _binitialoverlap _time _distance _location _impactpoint _normal _impactnormal _physmat _hitactor _hitcomponent) (`GameplayStatics.BreakHitResult` SweepResult))
  (bind _returnvalue (`KismetMathLibrary.Conv_VectorToRotator` _normal))
  (if (`ActorComponent.ComponentHasTag` OtherComp "Player")
    (`|ExecutionSequence` :!label _label
      (:`then_0`
        (if (!= OtherActor (`self.GetOwner` (`self.WeaponOwner`)))
          (`GameplayStatics.ApplyPointDamage` OtherActor (`self.BulletTypeCal` (`self.ProjectileID`)) (`.ImpactPoint` (`GameplayStatics.BreakHitResult` SweepResult)) SweepResult null (`self.WeaponOwner`))))
      (:`then_1`
        (`self.K2_DestroyActor`)))
    (else
      (switch `ECollisionChannel` (`PrimitiveComponent.GetCollisionObjectType` OtherComp)
        (:`ECC_WorldStatic`
          (`|ExecutionSequence`
            (:`then_0`
              (`GameplayStatics.PlaySoundAtLocation` "/Game/_Game/MyNew/Sound/Weapon/BulletHit/bullethit_metal_Cue.bullethit_metal_Cue" _impactpoint (struct) 1.0 1.0 0.0 null null null null)
              (`GameplayStatics.SpawnEmitterAttached` "/Game/Realistic_Starter_VFX_Pack_Vol2/Particles/Hit/P_Default.P_Default" _hitcomponent "None" _impactpoint _returnvalue (1.0 1.0 1.0) "KeepWorldPosition")
              (bind _returnvalue_2 (`GameplayStatics.SpawnDecalAttached` "/Game/_Game/MyNew/PJH/BP/Weapons/M_Decal1.M_Decal1" (15.0 3.0 3.0) _hitcomponent "None" _impactpoint _returnvalue "KeepWorldPosition" 10.0))
              (bind _decalsize_x (`KismetMathLibrary.BreakVector` (`DecalComponent.DecalSize` _returnvalue_2)))
              (`SceneComponent.K2_SetWorldLocation` _returnvalue_2 (- (`SceneComponent.K2_GetComponentLocation` _returnvalue_2) (* (* _decalsize_x 0.75) (* _normal 1.0))) false false))
            (:`then_1`
              (`self.K2_DestroyActor`))))
        (:`ECC_WorldDynamic`
          (goto _label))
        (:`ECC_Pawn`
          (goto _label))
        (:`ECC_GameTraceChannel1`
          (goto _label))))))

(fn `BulletTypeCal`
  (params (BulletType :type Name))
  (returns (Damage :type "Float (double-precision)"))
  (switch `name` BulletType
    (:`Default`
      (return 10.0))
    (:`9x19`
      (return 20.0))
    (:`545x39`
      (return 25.0))
    (:`762x39`
      (return 30.0))
    (:`ShotgunShell`
      (return 50.0))
    (:`ShotgunSlug`
      (return 80.0))))

(fn `UserConstructionScript`
  (bind _projectilemovement (`self.ProjectileMovement`))
  (`self.SetLifeSpan` (`self.LifeSpan`))
  (set `ProjectileMovementComponent.InitialSpeed` (* (`self.Velocity`) 100.0) _projectilemovement)
  (set `ProjectileMovementComponent.ProjectileGravityScale` (`self.Gravity`) _projectilemovement))