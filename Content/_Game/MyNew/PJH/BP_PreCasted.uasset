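; BP_PreCasted is a helper function set that returns commonly used game objects already cast to their project types.
; It casts the game mode, game instance and player 0's pawn to the project's Blueprint classes.
; The main inventory and main overlay widget getters build on the pawn getter, reading references from the character or its BPMultiplayer member.
; A separate utility swaps two floats by reference through a temporary value.
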(fn `CastedGameinstance`
  (returns (`AsBP Game Instance` :type "/Game/_Game/MyNew/PJH/BP_GameInstance Object Reference"))
  (bind _asbp_game_instance (cast `/Game/_Game/MyNew/PJH/BP_GameInstance` (`GameplayStatics.GetGameInstance` (`local.__WorldContext`))))
  (return _asbp_game_instance))

(fn `CastedGameMode`
  (returns (`BP MPGame Mode` :type "/Game/_Game/JigSInventory/Demo/BP_MPGameMode Object Reference"))
  (bind _asbp_mpgame_mode (cast `/Game/_Game/JigSInventory/Demo/BP_MPGameMode` (`GameplayStatics.GetGameMode` (`local.__WorldContext`))))
  (return _asbp_mpgame_mode))

(fn `CastedMainInventory`
  (returns (`BP Main Inventory` :type "/Game/_Game/MyNew/PJH/BP/Widget/BP_MainInventory Object Reference"))
  (bind _asbp_main_inventory (cast `/Game/_Game/MyNew/PJH/BP/Widget/BP_MainInventory` (`/Game/_Game/JigSInventory/Jigsaw/Components/BP_Multiplayer.InventoryWidgetRef` (`/Game/_Game/MyNew/PJH/BP/Charactor/Player/BP_MainChar.BP_Multiplayer` (`self.CastedPawn` (`local.__WorldContext`))))))
  (return _asbp_main_inventory))

(fn `CastedMainOverlay`
  (returns (WBP_MainOverlay :type "/Game/_Game/MyNew/PJH/BP/Widget/WBP_MainOverlay Object Reference"))
  (return (`/Game/_Game/MyNew/PJH/BP/Charactor/Player/BP_MainChar.WBP_MainOverlay` (`self.CastedPawn` (`local.__WorldContext`)))))

(fn `CastedPawn`
  (returns (`BP Main Char` :type "/Game/_Game/MyNew/PJH/BP/Charactor/Player/BP_MainChar Object Reference"))
  (bind _asbp_main_char (cast `/Game/_Game/MyNew/PJH/BP/Charactor/Player/BP_MainChar` (`GameplayStatics.GetPlayerPawn` (`local.__WorldContext`))))
  (return _asbp_main_char))

(fn `Swap_Float`
  (params (A :type "Float (double-precision) (by ref)") (B :type "Float (double-precision) (by ref)"))
  (returns (SwapedA :type "Float (double-precision)") (SwapedB :type "Float (double-precision)"))
  (locals (Temp :type "Float (double-precision)") (TempB :type Integer))
  (set `local.Temp` A)
  (`|VariableSetRef` A (`local.B`))
  (`|VariableSetRef` (`local.B`) (`local.Temp`))
  (return (`local.A`) (`local.B`)))