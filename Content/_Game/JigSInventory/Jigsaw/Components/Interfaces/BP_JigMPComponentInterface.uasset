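; BP_JigMPComponentInterface is a Blueprint interface for JigMP components in the Jigsaw inventory system, declaring inventory event callbacks and a loot widget getter.
; Callbacks cover item add, remove, move, drop and consume, pickup add and equip, container swaps and chamber UID updates.
; Payloads identify items and containers mainly by UID, with names, item info, components or actors where relevant.
; It holds only signatures, leaving behavior to implementers.
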(fn `JigMP_GetLootWidget`
  (returns (Result :type "Widget Object Reference") (`Valid?` :type Boolean))
  (return null false))

(fn `JigMP_OnContainersSwap`
  (params (Container1 :type "/Game/_Game/JigSInventory/Jigsaw/Widgets/WBP_Container Object Reference") (Container2 :type "/Game/_Game/JigSInventory/Jigsaw/Widgets/WBP_Container Object Reference"))
  (returns (Result :type Boolean))
  (return false))

(fn `JigMP_OnItemAdded`
  (params (ItemUID :type "Guid Structure") (FromContainerUID :type "Guid Structure") (ToContainerUID :type "Guid Structure") (FromComponent :type "/Game/_Game/JigSInventory/Jigsaw/Components/BP_Multiplayer Object Reference"))
  (returns (Result :type Boolean))
  (return false))

(fn `JigMP_OnItemConsumed`
  (params (ConsumedItem :type "/Game/_Game/JigSInventory/Jigsaw/Data/RepItemInfo Structure") (Amount :type Integer) (Remaining :type Integer) (InsideOf :type "/Game/_Game/JigSInventory/Jigsaw/Data/RepItemInfo Structure") (FromContainer :type Name) (CustomData :type String))
  (returns (Result :type Boolean))
  (return false))

(fn `JigMP_OnItemDropped`
  (params (ItemUID :type "Guid Structure") (FromContainerUID :type "Guid Structure") (ActorRef :type "Actor Object Reference"))
  (returns (Result :type Boolean))
  (return false))

(fn `JigMP_OnItemMoved`
  (params (ItemUID :type "Guid Structure") (FromContainerUID :type "Guid Structure") (ToContainerUID :type "Guid Structure"))
  (returns (Result :type Boolean))
  (return false))

(fn `JigMP_OnItemRemoved`
  (params (ItemUID :type "Guid Structure") (FromContainerUID :type "Guid Structure") (ToContainerUID :type "Guid Structure") (ToComponent :type "/Game/_Game/JigSInventory/Jigsaw/Components/BP_Multiplayer Object Reference"))
  (returns (Result :type Boolean))
  (return false))

(fn `JigMP_OnMainContainerItemAdded`
  (params (ToContainerUID :type "Guid Structure") (ItemUID :type "Guid Structure") (ToContainerName :type Name) (ItemInfo :type "/Game/_Game/JigSInventory/Jigsaw/Data/RepItemInfo Structure") (FromMain :type Name))
  (returns (Result :type Boolean) (ActorRef :type "Actor Object Reference"))
  (return false null))

(fn `JigMP_OnMainContainerItemRemoved`
  (params (FromContainerUID :type "Guid Structure") (ItemUID :type "Guid Structure") (ContainerName :type Name) (ItemRemovedInfo :type "/Game/_Game/JigSInventory/Jigsaw/Data/RepItemInfo Structure"))
  (returns (Result :type Boolean))
  (return false))

(fn `JigMP_OnPickupAdded`
  (params (Info :type "/Game/_Game/JigSInventory/Jigsaw/Data/RepItemInfo Structure") (ItemUID :type "Guid Structure") (ToContainerUID :type "Guid Structure") (ToContainer :type Name))
  (returns (Result :type Boolean))
  (return false))

(fn `JigMP_OnPickupEquipped`
  (params (ActorRef :type "Actor Object Reference") (ToContainerName :type Name) (UID :type "Guid Structure") (ToContainerUID :type "Guid Structure") (Info :type "/Game/_Game/JigSInventory/Jigsaw/Data/RepItemInfo Structure"))
  (returns (Result :type Boolean))
  (return false))

(fn `JigMP_OnRequestDropItem`
  (params (ItemInfo :type "/Game/_Game/JigSInventory/Jigsaw/Data/RepItemInfo Structure") (ContainerName :type Name) (FromJSI :type "/Game/_Game/JigSInventory/Jigsaw/Widgets/WBP_Container Object Reference"))
  (returns (ActorRef :type "Actor Object Reference"))
  (return null))

(fn `JigMP_OnTwoContainersSwap`
  (params (FromContainer :type Name) (ToContainer :type Name))
  (returns (Result :type Boolean))
  (return false))

(fn `JigMP_OnUpdateChamberUID`
  (params (NewUID :type "Guid Structure"))
  (returns (Result :type Boolean))
  (return false))