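; Pickup component for the Jigsaw inventory that makes its owning actor an interactable item or lootable container.
; On authority, it restores count or builds starting containers through the owner's BP_Multiplayer component, then sets up physics and attachments.
; Interaction forwards pickup or opens a loot widget, hiding unrevealed contents and closing by distance timer.
; Replicated attachment data drives locally spawned attachment actors, socketed by parent UID and container index, skipped on dedicated servers.
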(event `self.ReceiveBeginPlay`
  (bind (_returnvalue _pickupinfo) (`/Game/_Game/JigSInventory/Jigsaw/Components/BP_Multiplayer.IsValidPickup` (`self.OwnerMPComp`)))
  ;[0.06771 0.06771 0.06771] Process attachments
  (`parent.ReceiveBeginPlay`)
  (`self.GetMPComp`
    (:`Found`
      (if (`Actor.HasAuthority` (`self.GetOwner`))
        (`|ExecutionSequence`
          (:`then_0`
            (`KismetSystemLibrary.Delay` 0.01)
            (if _returnvalue
              (`self.SetCount` (`.Count_8_DD79AF2A46126A338C8DCCB4616D91CD` (break `/Game/_Game/JigSInventory/Jigsaw/Data/ST_RepItemInfo` (`.ItemInfo_25_937A083B4BD3D9B590E0A69C76A4F6F7` (break `/Game/_Game/JigSInventory/Jigsaw/Data/ST_ContainerPickupsInfo` _pickupinfo)))))
              (elif (`self.CanBePicked?`)
                (`self.ProcessStartingItems` (`self.OwnerMPComp`)))))
          (:`then_1`
            (`KismetSystemLibrary.Delay` 0.1)
            (if (and (`self.CanBePicked?`) (`self.EnablePhysics?`))
              (`PrimitiveComponent.SetSimulatePhysics` (cast `PrimitiveComponent` (`Actor.RootComponent` (`self.GetOwner`)) :!pure true) true))
            (`self.UpdateAttachments`)))))))

(event `OnExecuteInteract`
  (params (Actor :type "Actor Object Reference") (Option :type "/Game/_Game/JigSInventory/Jigsaw/Components/Interfaces/E_InteractOptions Enum" :default "NewEnumerator0"))
  (bind _ownermpcomp (`self.OwnerMPComp`))
  ;[0.06771 0.06771 0.06771] Handle interaction
  (if (or (`|EnumEquality` Option "NewEnumerator0") (not (`/Game/_Game/JigSInventory/Jigsaw/Components/BP_Multiplayer.CanLootPickup?` (`self.OwnerMPComp`))))
    (message `/Game/_Game/JigSInventory/Jigsaw/Components/Interfaces/BP_JigCharacterInterface.OnPickupInteractExecuted` Actor (`self.GetOwner`))
    (else
      (set `self.CurrentActor` Actor)
      (if (not (`/Game/_Game/JigSInventory/Jigsaw/Components/BP_Multiplayer.IsInventoryVisible?` _ownermpcomp))
        (bind _inventorywidgetref (`/Game/_Game/JigSInventory/Jigsaw/Components/BP_Multiplayer.SetupInventoryWidget` _ownermpcomp true false))
        (bind _output_get (set `self.Inventory Widget Ref` _inventorywidgetref))
        (`self.SetHide` _output_get)
        (message `/Game/_Game/JigSInventory/Jigsaw/Components/Interfaces/BP_JigCharacterInterface.AddJigWidgetToContent` Actor _output_get (`/Game/_Game/JigSInventory/Jigsaw/Data/DataAsset/JigsawItem_DataAsset.Name` (`self.ItemDataAsset`)))
        (message `/Game/_Game/JigSInventory/Jigsaw/Components/Interfaces/BP_JigCharacterInterface.RequestServerData` Actor (`self.OwnerMPComp`))
        (`self.SetInteractDistance` (`self.CurrentActor`))
        (`KismetSystemLibrary.K2_SetTimer` null "CheckDistanceFromActor" 0.1 true)))))

(event `CustomTick`)

(event `self.ReceiveEndPlay`
  (params (EndPlayReason :type "EEndPlayReason Enum" :default "Destroyed"))
  ;[0.06771 0.06771 0.06771] When owner is destroyed also destroy its attachments
  (`parent.ReceiveEndPlay` EndPlayReason)
  (for _array_element (`self.InstalledAttachments`)
    (`Actor.K2_DestroyActor` _array_element))
  (`/Engine/EditorBlueprintResources/StandardMacros.IsValid` (`self.CurrentActor`)
    (:`Is Valid`
      (message `/Game/_Game/JigSInventory/Jigsaw/Components/Interfaces/BP_JigCharacterInterface.OnInteractActorOverDistance` (`self.CurrentActor`) (`self.GetOwner`)))))

(fn `CanInteract?`
  (returns (`CanBePicked?` :type Boolean))
  (return (`self.CanBePicked?`)))

(fn `CheckDistanceFromActor`
  (bind _currentactor (`self.CurrentActor`))
  ;[0.151 0.151 0.151] Close the loot container widget if the player is too far
  (`/Engine/EditorBlueprintResources/StandardMacros.IsValid` _currentactor
    (:`Is Valid`
      (if (> (`KismetMathLibrary.VSize` (- (`self.InteractingActorLoc`) (`Actor.K2_GetActorLocation` _currentactor))) 300.0)
        (`KismetSystemLibrary.K2_ClearTimer` null "CheckDistanceFromActor")
        (message `/Game/_Game/JigSInventory/Jigsaw/Components/Interfaces/BP_JigCharacterInterface.OnInteractActorOverDistance` (`self.CurrentActor`) (`self.GetOwner`))
        (set `self.CurrentActor` null)))
    (:`Is Not Valid`
      (`KismetSystemLibrary.K2_ClearTimer` null "CheckDistanceFromActor"))))

(fn `FindAttachmentByType`
  (params (Type :type "/Game/_Game/JigSInventory/Jigsaw/Data/AttachmentType Enum" :default "NewEnumerator9"))
  (returns (Attachment :type "/Game/_Game/JigSInventory/Jigsaw/Pickup/BP_AMainLocalAttachment Object Reference") (Found :type Boolean))
  (for _array_element (`self.InstalledAttachments`)
    (bind (_uid _attachmentinfo) (`/Game/_Game/JigSInventory/Jigsaw/Pickup/BP_WeaponAttachments.Jig_GetAttachmentInfo` _array_element))
    (if (`|EnumEquality` (`/Game/_Game/JigSInventory/Jigsaw/Data/DataAsset/JigsawItem_DataAsset.Local_AttachmentType` _attachmentinfo) Type)
      (return _array_element true)))
  (return null false))

(fn `FindAttachmentByTypeArr`
  (params (Type :type "/Game/_Game/JigSInventory/Jigsaw/Data/AttachmentType Enum" :default "NewEnumerator9"))
  (returns (Attachment :type "Array of /Game/_Game/JigSInventory/Jigsaw/Pickup/BP_AMainLocalAttachment Object Reference") (Found :type Boolean))
  (locals (Arr :type "Array of /Game/_Game/JigSInventory/Jigsaw/Pickup/BP_AMainLocalAttachment Object Reference"))
  (bind _arr (`local.Arr`))
  (for _array_element (`self.InstalledAttachments`)
    (bind (_uid _attachmentinfo) (`/Game/_Game/JigSInventory/Jigsaw/Pickup/BP_WeaponAttachments.Jig_GetAttachmentInfo` _array_element))
    (if (`|EnumEquality` (`/Game/_Game/JigSInventory/Jigsaw/Data/DataAsset/JigsawItem_DataAsset.Local_AttachmentType` _attachmentinfo) Type)
      (`KismetArrayLibrary.Array_AddUnique` (`local.Arr`) _array_element)))
  (return _arr (`KismetArrayLibrary.Array_IsValidIndex` _arr)))

(fn `FindLocalAttachmentByUID`
  (params (UID :type "Guid Structure"))
  (returns (Attachment :type "/Game/_Game/JigSInventory/Jigsaw/Pickup/BP_AMainLocalAttachment Object Reference"))
  (for _array_element (`self.InstalledAttachments`)
    (bind _uid (message `/Game/_Game/JigSInventory/Jigsaw/Pickup/BP_WeaponAttachments.Jig_GetAttachmentInfo` _array_element))
    (if (== _uid (`local.UID`))
      (return _array_element)))
  (return null))

(fn `GetAttachSocketByInContainerIndex`
  (params (Info :type "/Game/_Game/JigSInventory/Jigsaw/Data/DataAsset/JigsawItem_DataAsset Object Reference") (InContainerIndex :type Integer))
  (returns (Socket :type Name))
  ;[1 1 1] In container index: Take a handguard for example, a laser sight could be installed to the left or the right side, so we determine the socket based on InContainerIndex.
  ; This depends on how you setup your special container.
  (`|ExecutionSequence`
    (:`then_0`
      (for _array_element (`/Game/_Game/JigSInventory/Jigsaw/Data/DataAsset/JigsawItem_DataAsset.Local_AttachToSocketByContainerIndex` Info)
        (bind (_index _socketname) (break `/Game/_Game/JigSInventory/Jigsaw/Pickup/ST_LocalAttContainerIndexSocket` _array_element))
        (if (== _index (`local.InContainerIndex`))
          (return _socketname))))
    (:`then_1`
      (return (`/Game/_Game/JigSInventory/Jigsaw/Data/DataAsset/JigsawItem_DataAsset.Local_AttachSocket` Info)))))

(fn `GetCount`
  (returns (Count :type Integer))
  (if (< (`self.OverrideCount`) 0)
    (return (`/Game/_Game/JigSInventory/Jigsaw/Data/DataAsset/JigsawItem_DataAsset.Count` (`self.ItemDataAsset`)))
    (else
      (return (`self.OverrideCount`)))))

(fn `GetPickupName`
  (returns (Result :type Text))
  (bind _count (`self.GetCount`))
  (return (`KismetTextLibrary.Conv_StringToText` (`KismetStringLibrary.Concat_StrStr` (`KismetTextLibrary.Conv_TextToString` (`/Game/_Game/JigSInventory/Jigsaw/Data/DataAsset/JigsawItem_DataAsset.Name` (`self.ItemDataAsset`))) (`KismetMathLibrary.SelectString` (`KismetStringLibrary.Concat_StrStr` " x" (`KismetStringLibrary.Conv_IntToString` _count)) "" (> _count 1))))))

(fn `HideWidget`
  (params (Widget :type "Object Object Reference"))
  (returns (Success :type Boolean))
  (return false))

(fn `ModifyDurability`
  (params (Durability :type "Float (double-precision)"))
  (locals (Info :type "/Game/_Game/JigSInventory/Jigsaw/Data/ST_ContainerPickupsInfo Structure"))
  (bind _ownermpcomp (`self.OwnerMPComp`))
  (bind (_returnvalue _pickupinfo) (`/Game/_Game/JigSInventory/Jigsaw/Components/BP_Multiplayer.IsValidPickup` (`self.OwnerMPComp`)))
  (if _returnvalue
    (bind _output_get (set `local.Info` _pickupinfo))
    (bind ((`ItemInfo_25_937A083B4BD3D9B590E0A69C76A4F6F7` _iteminfo)) (break `/Game/_Game/JigSInventory/Jigsaw/Data/ST_ContainerPickupsInfo` _output_get))
    (setmembers `/Game/_Game/JigSInventory/Jigsaw/Data/ST_RepItemInfo` :`StructRef` _iteminfo :`Durability` (`KismetMathLibrary.MakeVector2D` Durability (`.Y` (`KismetMathLibrary.BreakVector2D` (`.Durability_22_A3557C454274D193D47AB9B71FB0C0CA` (break `/Game/_Game/JigSInventory/Jigsaw/Data/ST_RepItemInfo` _iteminfo))))))
    (`/Game/_Game/JigSInventory/Jigsaw/Components/BP_Multiplayer.SetPickupContainerData` _ownermpcomp (`local.Info`) (`/Game/_Game/JigSInventory/Jigsaw/Components/BP_Multiplayer.MainContainers` _ownermpcomp))))

(fn `OnAttachmentInstalled`
  (params (MainUID :type "Guid Structure") (Attachments :type "Array of /Game/_Game/JigSInventory/Jigsaw/Data/ST_RepAttachmentInfo Structure (by ref)"))
  (set `self.RepAttachments` (make `/Game/_Game/JigSInventory/Jigsaw/Data/ST_RepWeaponAttachment` MainUID Attachments))
  (`self.ProcessAttachments`))

(fn `OnRep_CanEquip?`
  (`/Engine/EditorBlueprintResources/StandardMacros.IsValid` (`self.CurrentActor`)
    (:`Is Valid`
      (`KismetSystemLibrary.K2_ClearTimer` null "CheckDistanceFromActor")
      (message `/Game/_Game/JigSInventory/Jigsaw/Components/Interfaces/BP_JigCharacterInterface.OnInteractActorOverDistance` (`self.CurrentActor`) (`self.GetOwner`))
      (set `self.CurrentActor` null))))

(fn `OnRep_EnablePhysics?`)

(fn `OnRep_RepAttachments`
  ;[1 1 1] Only process attachments if we are not a dedicated server or listen server, the latter already has.
  (if (and (not (`KismetSystemLibrary.IsDedicatedServer`)) (not (`Actor.HasAuthority` (`self.GetOwner`))))
    (`self.ProcessAttachments`)))

(fn `ProcessAttachments`
  (locals (AttachmentRef :type "/Game/_Game/JigSInventory/Jigsaw/Pickup/BP_AMainLocalAttachment Object Reference") (CurrentInfo :type "/Game/_Game/JigSInventory/Jigsaw/Data/ST_RepAttachmentInfo Structure") (TempInstalledAttachments :type "Array of Actor Object Reference"))
  (bind _attachmentref (`local.AttachmentRef`))
  (bind ((`AttachmentContainerIndex_14_13E8F2B740F8A6C0E8AF539039840CA2` _attachmentcontainerindex) (`ParentUID_20_9FAD2D1149DFF8D1239C3F90FFDE2A2C` _parentuid)) (break `/Game/_Game/JigSInventory/Jigsaw/Data/ST_RepAttachmentInfo` (`local.CurrentInfo`)))
  ;[1 1 1] Process attachments
  (if (`self.ProcessAttachments?`)
    (if (not (`KismetSystemLibrary.IsDedicatedServer`))
      (for _array_element (`.Attachments_6_38F2C7B64C1B85D80C3C35A8B1026969` (break `/Game/_Game/JigSInventory/Jigsaw/Data/ST_RepWeaponAttachment` (`self.RepAttachments`)))
        (set `local.CurrentInfo` _array_element)
        (bind ((`AttachmentID_21_84163C9E4A907293E46F1888C9CBB5C8` _attachmentid) (`AttachmentUID_19_C9C3B4D343E900A444D5DD870C104204` _attachmentuid)) (break `/Game/_Game/JigSInventory/Jigsaw/Data/ST_RepAttachmentInfo` _array_element))
        (bind _attachment (`self.FindLocalAttachmentByUID` _attachmentuid))
        (bind _output_get (set `local.AttachmentRef` _attachment))
        (`|ExecutionSequence`
          (:`then_0`
            (`/Engine/EditorBlueprintResources/StandardMacros.IsValid` _output_get
              (:`Is Not Valid`
                (bind _local_actorclass (`/Game/_Game/JigSInventory/Jigsaw/Data/DataAsset/JigsawItem_DataAsset.Local_ActorClass` _attachmentid))
                (if (`KismetSystemLibrary.IsValidClass` _local_actorclass)
                  (bind _returnvalue (`|SpawnActorFromClass` _local_actorclass (`KismetMathLibrary.MakeTransform` (`Actor.K2_GetActorLocation` (`self.GetOwner`))) "AdjustIfPossibleButAlwaysSpawn" "OverrideRootScale" null null))
                  (bind _output_get_2 (set `local.AttachmentRef` _returnvalue))
                  (message `/Game/_Game/JigSInventory/Jigsaw/Pickup/BP_WeaponAttachments.Jig_SetAttachmentInfo` _output_get_2 (`.AttachmentUID_19_C9C3B4D343E900A444D5DD870C104204` (break `/Game/_Game/JigSInventory/Jigsaw/Data/ST_RepAttachmentInfo` (`local.CurrentInfo`))) _attachmentid)))))
          (:`then_1`
            (`/Engine/EditorBlueprintResources/StandardMacros.IsValid` _output_get
              (:`Is Valid`
                (`KismetArrayLibrary.Array_Add` (`local.TempInstalledAttachments`) (`local.AttachmentRef`))
                (if (== (`.MainUID_7_3F7D5E5149793F902437078F3B35819D` (break `/Game/_Game/JigSInventory/Jigsaw/Data/ST_RepWeaponAttachment` (`self.RepAttachments`))) _parentuid)
                  (bind (_uid _attachmentinfo) (message `/Game/_Game/JigSInventory/Jigsaw/Pickup/BP_WeaponAttachments.Jig_GetAttachmentInfo` (`local.AttachmentRef`)))
                  (`Actor.K2_AttachToComponent` (`local.AttachmentRef`) (`Actor.RootComponent` (`self.GetOwner`)) (`/Game/_Game/JigSInventory/Jigsaw/Data/DataAsset/JigsawItem_DataAsset.Local_AttachSocket` _attachmentinfo) "SnapToTarget" "SnapToTarget" "KeepWorld" true)
                  (`KismetArrayLibrary.Array_AddUnique` (`self.InstalledAttachments`) (`local.AttachmentRef`) :!label _label)
                  (else
                    (bind _attachment_2 (`self.FindLocalAttachmentByUID` _parentuid))
                    (`/Engine/EditorBlueprintResources/StandardMacros.IsValid` _attachment_2
                      (:`Is Valid`
                        (bind (_uid_2 _attachmentinfo_2) (message `/Game/_Game/JigSInventory/Jigsaw/Pickup/BP_WeaponAttachments.Jig_GetAttachmentInfo` _attachmentref))
                        (bind _comp (`/Game/_Game/JigSInventory/Jigsaw/Pickup/BP_AMainLocalAttachment.Jig_GetPrimitiveComponent` _attachment_2))
                        (`Actor.K2_AttachToComponent` _attachmentref _comp (`self.GetAttachSocketByInContainerIndex` _attachmentinfo_2 _attachmentcontainerindex) "SnapToTarget" "SnapToTarget" "KeepWorld" true)
                        (goto _label))
                      (:`Is Not Valid`
                        (`KismetSystemLibrary.PrintString` "Failed to find parent attachment.." true true (struct :`R` 1.0 :`A` 1.0))
                        (`Actor.K2_DestroyActor` (`local.AttachmentRef`)))))))))))
      (bind (_arrayindex _arrayelement) (`/Engine/EditorBlueprintResources/StandardMacros.ReverseForEachLoop` (`self.InstalledAttachments`))
        (:`LoopBody`
          (if (not (`KismetArrayLibrary.Array_Contains` (`local.TempInstalledAttachments`) _arrayelement))
            (`Actor.K2_DestroyActor` _arrayelement)
            (`KismetArrayLibrary.Array_Remove` (`self.InstalledAttachments`) _arrayindex)))
        (:`Completed`
          (`self.OnAttachmentsUpdated`))))))

(fn `ProcessStartingItems`
  (params (MPComp :type "/Game/_Game/JigSInventory/Jigsaw/Components/BP_Multiplayer Object Reference"))
  (locals (NewUID :type "Guid Structure") (SubContainers :type "Array of /Game/_Game/JigSInventory/Jigsaw/Components/Data/ST_SubContainerInfo Structure") (MainContainerUIDs :type "Array of Guid Structure") (NewInfo :type "/Game/_Game/JigSInventory/Jigsaw/Data/ST_ContainerPickupsInfo Structure"))
  (bind _maincontaineruids (`local.MainContainerUIDs`))
  (bind _mpcomp (`local.MPComp`))
  (bind _mpcomp_2 (`local.MPComp`))
  (bind _itemdataasset (`self.ItemDataAsset`))
  (bind _maincontainers (`/Game/_Game/JigSInventory/Jigsaw/Components/BP_Multiplayer.MainContainers` _mpcomp_2))
  ;[0.04688 0.04688 0.04688] Process pickup starting items
  (if (> (`KismetArrayLibrary.Array_Length` (`/Game/_Game/JigSInventory/Jigsaw/Components/BP_Multiplayer.ContainersSettings` MPComp)) 0)
    (set `local.NewUID` (`/Game/_Game/JigSInventory/Jigsaw/Components/BP_Multiplayer.GetUniqueID` _mpcomp))
    (for (_array_element _array_index) (`/Game/_Game/JigSInventory/Jigsaw/Components/BP_Multiplayer.ContainersSettings` _mpcomp)
      (bind ((`IsEquipTo?_17_A70EBD1B42E398B0EB14E0B352CCC0A2` _isequipto_) (`Columns_4_A32AA159420F47D951669C9636084F9D` _columns) (`Rows_6_E1A84D8A441B19CA3C38D0BC029805A1` _rows) (`StartingItems_10_C6DB208442353E0AA9B5DB892266821A` _startingitems)) (break `/Game/_Game/JigSInventory/Jigsaw/Components/Data/ST_JigCompContentSettings` _array_element))
      (bind _contuid (`/Game/_Game/JigSInventory/Jigsaw/Components/BP_Multiplayer.ReplicateContainer` (`local.MPComp`) "None" _isequipto_ _columns _rows _startingitems "NewEnumerator0" false))
      (`KismetArrayLibrary.Array_Add` (`local.MainContainerUIDs`) _contuid)
      (`KismetArrayLibrary.Array_Add` (`local.SubContainers`) (make `/Game/_Game/JigSInventory/Jigsaw/Components/Data/ST_SubContainerInfo` (`local.NewUID`) _array_index _contuid)))
    (set `local.NewInfo` (make `/Game/_Game/JigSInventory/Jigsaw/Data/ST_ContainerPickupsInfo` (`local.NewUID`) true (0.0 0.0) (make `/Game/_Game/JigSInventory/Jigsaw/Data/ST_RepItemInfo` (`self.ItemDataAsset`) 1 (`/Game/_Game/JigSInventory/Jigsaw/Data/DataAsset/JigsawItem_DataAsset.SlotDimensions` _itemdataasset) (`/Game/_Game/JigSInventory/Jigsaw/Data/DataAsset/JigsawItem_DataAsset.Weight` _itemdataasset) (`/Game/_Game/JigSInventory/Jigsaw/Data/DataAsset/JigsawItem_DataAsset.Price` _itemdataasset) (`KismetMathLibrary.MakeVector2D` (`/Game/_Game/JigSInventory/Jigsaw/Data/DataAsset/JigsawItem_DataAsset.Durability` _itemdataasset) (`/Game/_Game/JigSInventory/Jigsaw/Data/DataAsset/JigsawItem_DataAsset.MaxDurability` _itemdataasset)) (`/Game/_Game/JigSInventory/Jigsaw/Components/BP_Multiplayer.GenerateRandomStats` (`local.MPComp`) (`self.RandomStatConfig`) (`/Game/_Game/JigSInventory/Jigsaw/Data/DataAsset/JigsawItem_DataAsset.ItemStats` _itemdataasset))) "00000000000000000000000000000000" -1 false 0 null (`local.SubContainers`)))
    (for (_array_element_2 _array_index_2) _maincontainers
      (bind ((`ReplicationUID_23_EB27D09649B6E02591DCA98708B06332` _replicationuid)) (break `/Game/_Game/JigSInventory/Jigsaw/Components/Data/ST_ReplicatedContainerInfo` _array_element_2))
      (if (`KismetArrayLibrary.Array_Contains` _maincontaineruids _replicationuid)
        (setmembers `/Game/_Game/JigSInventory/Jigsaw/Components/Data/ST_ReplicatedContainerInfo` :`StructRef` (`|GetArrayItem` _maincontainers _array_index_2) :`InContainerUID` (`local.NewUID`) :`ContainerIndex` (`KismetArrayLibrary.Array_Find` _maincontaineruids _replicationuid))))
    (`/Game/_Game/JigSInventory/Jigsaw/Components/BP_Multiplayer.SetPickupContainerData` _mpcomp_2 (`local.NewInfo`) _maincontainers)))

(fn `SetCanInteract`
  (params (CanInteract :type Boolean) (EnablePhysics :type Boolean))
  (returns (Result :type Boolean))
  ;[0.151 0.151 0.151] When this pickup gets equipped, disable physics and interaction
  (bind _output_get (set `self.CanBePicked?` CanInteract))
  (bind _output_get_2 (set `self.EnablePhysics?` EnablePhysics))
  (`PrimitiveComponent.SetSimulatePhysics` (cast `PrimitiveComponent` (`Actor.RootComponent` (`self.GetOwner`)) :!pure true) _output_get_2)
  (return _output_get))

(fn `SetCount`
  (params (OverrideCount :type Integer))
  (set `self.OverrideCount` OverrideCount))

(fn `SetHide`
  (params (Widget :type "UserWidget Object Reference"))
  (if (not (`self.IsRevealed`))
    (bind _aswbp_slot_root (cast `/Game/_Game/MyNew/PJH/BP/WBP_SlotRoot` Widget))
    (set `/Game/_Game/MyNew/PJH/BP/WBP_SlotRoot.ParentObject` self _aswbp_slot_root)
    (`/Game/_Game/MyNew/PJH/BP/WBP_SlotRoot.HideContents` _aswbp_slot_root)))

(fn `SetInteractDistance`
  (params (Target :type "Actor Object Reference"))
  ;[0.07292 0.07292 0.07292] Set the distance from the interact object the moment of the interaction
  (set `self.InteractingActorLoc` (`Actor.K2_GetActorLocation` Target)))

(fn `SetReveal`
  (params (SetIsReveal :type Boolean) (GUID :type "Guid Structure") (ItemRef :type "/Game/_Game/JigSInventory/Jigsaw/Widgets/BP_Slot Object Reference"))
  (returns (Return :type Boolean))
  (bind _output_get (set `self.IsRevealed` SetIsReveal))
  (return _output_get))

(fn `Unhide_eachSlot`
  (returns (AllSearched :type Boolean))
  (bind _containers (message `/Game/_Game/JigSInventory/Jigsaw/Widgets/SpecialContainers/BP_IF_SpecialWidgetInterface.GetListOfContainers` (`self.Inventory Widget Ref`)))
  (for _array_element _containers
    (for _array_element_2 (`/Game/_Game/JigSInventory/Jigsaw/Widgets/WBP_Container.ArrayOfItems` _array_element)
      (if (`/Game/_Game/JigSInventory/Jigsaw/Widgets/BP_Slot.PJHSlotHidden` _array_element_2)
        (bind _jigcomp (message `/Game/_Game/JigSInventory/Jigsaw/Components/Interfaces/BP_MpInteractInterface.GetMultiplayerComponent` (`self.GetOwner`)))
        (`/Game/_Game/JigSInventory/Jigsaw/Components/BP_Multiplayer.SetHiddenItemsBySlotUID` _jigcomp (`/Game/_Game/JigSInventory/Jigsaw/Widgets/BP_Slot.ItemUniqueID` _array_element_2))
        (`/Game/_Game/JigSInventory/Jigsaw/Widgets/BP_Slot.UnHide` _array_element_2)
        (return false))))
  (return true))

(fn `UpdateAttachments`
  (bind _ownermpcomp (`self.OwnerMPComp`))
  (bind (_returnvalue _pickupinfo) (`/Game/_Game/JigSInventory/Jigsaw/Components/BP_Multiplayer.IsValidPickup` _ownermpcomp))
  (bind ((`UniqueServerID_37_C49AE0DA449ACAE3BE4633A263303B68` _uniqueserverid)) (break `/Game/_Game/JigSInventory/Jigsaw/Data/ST_ContainerPickupsInfo` _pickupinfo))
  (if (and _returnvalue (`self.CanBePicked?`) (`self.ProcessAttachments?`))
    (bind _attachments (`/Game/_Game/JigSInventory/Jigsaw/Components/BP_Multiplayer.GetListOfAttachments` _ownermpcomp _uniqueserverid))
    (set `self.RepAttachments` (make `/Game/_Game/JigSInventory/Jigsaw/Data/ST_RepWeaponAttachment` _uniqueserverid _attachments))
    (`self.ProcessAttachments`)))