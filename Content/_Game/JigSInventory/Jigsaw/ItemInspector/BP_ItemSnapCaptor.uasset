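; Scene capture actor that photographs Jigsaw inventory items into render targets for inventory and action bar images.
; It poses a static or skeletal mesh from the item's data asset, spawns socketed, nested attachments and captures only itself and those.
; Render targets are sized by slot dimensions and can be shared by item ID.
; Manual captures rely on post-process alpha, and CaptureFromTarget signals completion so the game state processes the next item.
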(event `self.ReceiveBeginPlay`
  (set `SceneCaptureComponent2D.FOVAngle` (`self.InitialFOV`) (`self.SceneCaptureComponent2D`))
  (set `SceneCaptureComponent.MaxViewDistanceOverride` 1000.0 (`self.SceneCaptureComponent2D`)))

(event `DelayedDelegate`
  ;[0.01042 0.005849 0] We're using a post process to generate an alpha channel, delay is needed to ensure the post process effect.
  ;
  ; Ignore inefficiency warning in log, even though we have captureEveryFrame set to true the SceneCapture is not ticking at all, we're using CaptureScene to capture manually once.
  ; For some reason captureEveryFrame has to be true for our post process to work but it has no effect on capturing.
  (`SceneCaptureComponent2D.CaptureScene` (`self.SceneCaptureComponent2D`))
  (set `SceneCaptureComponent2D.TextureTarget` null (`self.SceneCaptureComponent2D`))
  (`self.OnSnapTaken` :!pinned true) ; Tell the game state to process the next item\nYou can delay this call if you need more time
)

(fn `CaptureFromTarget`
  (params (TextureTarget :type "TextureRenderTarget2D Object Reference"))
  (set `SceneCaptureComponent2D.TextureTarget` TextureTarget (`self.SceneCaptureComponent2D`))
  (`self.DelayedDelegate`))

(fn `ClearAttachments`
  (bind _currentattachments (`self.CurrentAttachments`))
  (bind _showonlyactors (`SceneCaptureComponent.ShowOnlyActors` (`self.SceneCaptureComponent2D`)))
  (`KismetArrayLibrary.Array_Clear` _showonlyactors)
  (`KismetArrayLibrary.Array_Add` _showonlyactors self)
  (bind (_arrayindex _arrayelement) (`/Engine/EditorBlueprintResources/StandardMacros.ReverseForEachLoop` _currentattachments)
    (:`LoopBody`
      (`self.K2_DestroyActor` _arrayelement))
    (:`Completed`
      (`KismetArrayLibrary.Array_Clear` _currentattachments))))

(fn `GetActiveComponent`
  (returns (Comp :type "SceneComponent Object Reference"))
  (`/Engine/EditorBlueprintResources/StandardMacros.IsValid` (`StaticMeshComponent.StaticMesh` (`self.StaticMesh`))
    (:`Is Valid`
      (return (`self.StaticMesh`)))
    (:`Is Not Valid`
      (return (`self.SkeletalMesh`)))))

(fn `GetAttachSocketByInContainerIndex`
  (params (Info :type "/Game/_Game/JigSInventory/Jigsaw/Data/DataAsset/JigsawItem_DataAsset Object Reference") (InContainerIndex :type Integer))
  (returns (Socket :type Name))
  ;[1 1 1] In container index: Take a handguard for example, a laser sight could be installed to the left or the right side, so we determine the socket based on InContainerIndex.
  ; This depends on how you setup your special container.
  (`|ExecutionSequence`
    (:`then_0`
      (for _array_element (`/Game/_Game/JigSInventory/Jigsaw/Data/DataAsset/JigsawItem_DataAsset.Local_AttachToSocketByContainerIndex` Info)
        (bind (_index _socketname) (break `/Game/_Game/JigSInventory/Jigsaw/Pickup/S_LocalAttContainerIndexSocket` _array_element))
        (if (== _index (`local.InContainerIndex`))
          (return _socketname))))
    (:`then_1`
      (return (`/Game/_Game/JigSInventory/Jigsaw/Data/DataAsset/JigsawItem_DataAsset.Local_AttachSocket` Info)))))

(fn `GetDefaultDim`
  (params (Target :type "/Game/_Game/JigSInventory/Jigsaw/Widgets/BP_Slot Object Reference"))
  (returns (SlotDimension :type "Vector2D Structure"))
  (return (`/Game/_Game/JigSInventory/Jigsaw/Data/DataAsset/JigsawItem_DataAsset.SlotDimensions` (`/Game/_Game/JigSInventory/Jigsaw/Widgets/BP_Slot.GetJigDA` Target))))

(fn `GetInitValues`
  (returns (ReturnValue :type "Transform Structure") (FOVAngle :type "Float (double-precision)"))
  (bind _skeletalmesh (`self.SkeletalMesh`))
  (return (`SceneComponent.GetRelativeTransform` (select `bool` (`KismetSystemLibrary.IsValid` (`SkinnedMeshComponent.SkeletalMesh` _skeletalmesh)) :`false` (`self.StaticMesh`) :`true` _skeletalmesh :!type "SceneComponent Object Reference")) (`SceneCaptureComponent2D.FOVAngle` (`self.SceneCaptureComponent2D`))))

(fn `GetSnap`
  (params (ShareRTarget :type Boolean))
  (returns (Output_Get :type "TextureRenderTarget2D Object Reference") (`FromShared?` :type Boolean))
  (locals (RenderTarg :type "TextureRenderTarget2D Object Reference") (SaveRTarget :type Boolean))
  (bind _itemtoinspect (`self.ItemToInspect`))
  (bind _scenecapturecomponent2d (`self.SceneCaptureComponent2D`))
  (bind (_x _y) (`KismetMathLibrary.BreakVector2D` (select `bool` (`self.IsActionbar` _itemtoinspect) :`false` (* (`self.GetDefaultDim` _itemtoinspect) 90.0) :`true` (128.0 128.0))))
  (if ShareRTarget
    (bind _output_get (set `local.RenderTarg` (`BlueprintMapLibrary.Map_Find` (`self.CreatedRenderTargets`) (`/Game/_Game/JigSInventory/Jigsaw/Widgets/BP_Slot.GetItemID` _itemtoinspect))))
    (`/Engine/EditorBlueprintResources/StandardMacros.IsValid` _output_get
      (:`Is Valid`
        (return (`local.RenderTarg`) true))
      (:`Is Not Valid`
        (set `local.SaveRTarget` true)
        (bind _returnvalue (`KismetRenderingLibrary.CreateRenderTarget2D` (`KismetMathLibrary.FTrunc` _x) (`KismetMathLibrary.FTrunc` _y)))
        (bind _output_get_2 (set `local.RenderTarg` _returnvalue))
        (set `SceneCaptureComponent2D.TextureTarget` _output_get_2 (`self.SceneCaptureComponent2D`))
        (`SceneCaptureComponent2D.CaptureScene` _scenecapturecomponent2d)
        (set `SceneCaptureComponent2D.TextureTarget` null _scenecapturecomponent2d)
        (`|ExecutionSequence`
          (:`then_0`
            (if (`local.SaveRTarget`)
              (`BlueprintMapLibrary.Map_Add` (`self.CreatedRenderTargets`) (`/Game/_Game/JigSInventory/Jigsaw/Widgets/BP_Slot.GetItemID` (`self.ItemToInspect`)) (`local.RenderTarg`))))
          (:`then_1`
            (return (`local.RenderTarg`) false)))))))

(fn `GetSnapNoCapture`
  (params (Item :type "/Game/_Game/JigSInventory/Jigsaw/Widgets/BP_Slot Object Reference") (ShareRTarget :type Boolean))
  (returns (Output_Get :type "TextureRenderTarget2D Object Reference") (`FromShared?` :type Boolean))
  (locals (RenderTarg :type "TextureRenderTarget2D Object Reference") (SaveRTarget :type Boolean))
  (bind (_x _y) (`KismetMathLibrary.BreakVector2D` (select `bool` (`self.IsActionbar` Item) :`false` (* (`self.GetDefaultDim` Item) 120.0) :`true` (128.0 128.0))))
  (if ShareRTarget
    (bind _output_get (set `local.RenderTarg` (`BlueprintMapLibrary.Map_Find` (`self.CreatedRenderTargets`) (`/Game/_Game/JigSInventory/Jigsaw/Widgets/BP_Slot.GetItemID` Item))))
    (`/Engine/EditorBlueprintResources/StandardMacros.IsValid` _output_get
      (:`Is Valid`
        (return (`local.RenderTarg`) true))
      (:`Is Not Valid`
        (set `local.SaveRTarget` true))))
  (bind _returnvalue (`KismetRenderingLibrary.CreateRenderTarget2D` (`KismetMathLibrary.FTrunc` _x) (`KismetMathLibrary.FTrunc` _y)))
  (set `local.RenderTarg` _returnvalue)
  (`|ExecutionSequence`
    (:`then_0`
      (if (`local.SaveRTarget`)
        (`BlueprintMapLibrary.Map_Add` (`self.CreatedRenderTargets`) (`/Game/_Game/JigSInventory/Jigsaw/Widgets/BP_Slot.GetItemID` (`local.Item`)) (`local.RenderTarg`))))
    (:`then_1`
      (return (`local.RenderTarg`) false))))

(fn `InstallAttachments`
  (params (JigItem :type "/Game/_Game/JigSInventory/Jigsaw/Widgets/BP_Slot Object Reference"))
  (locals (AllAttachments :type "Array of /Game/_Game/JigSInventory/Jigsaw/Widgets/BP_Slot Object Reference") (CurrentJig :type "/Game/_Game/JigSInventory/Jigsaw/Widgets/BP_Slot Object Reference") (SpawnedItem :type "/Game/_Game/JigSInventory/Jigsaw/Pickup/BP_AMainLocalAttachment Object Reference") (LocalInfo :type "/Game/_Game/JigSInventory/Jigsaw/Data/DataAsset/JigsawItem_DataAsset Object Reference") (ParentUID :type "Guid Structure"))
  (bind _containerref (`/Game/_Game/JigSInventory/Jigsaw/Widgets/BP_Slot.GetContainerOneRef` JigItem))
  (`KismetArrayLibrary.Array_Clear` (`local.AllAttachments`))
  (`/Engine/EditorBlueprintResources/StandardMacros.IsValid` _containerref
    (:`Is Valid`
      (bind _containers (message `/Game/_Game/JigSInventory/Jigsaw/Widgets/SpecialContainers/BP_IF_SpecialWidgetInterface.GetListOfContainers` _containerref))
      (for _array_element _containers
        (if (`/Game/_Game/JigSInventory/Jigsaw/Widgets/WBP_Container.IsEquipTo?` _array_element)
          (`/Game/_Game/JigSInventory/Jigsaw/Widgets/WBP_Container.Deep_GettAllItems` _array_element (`local.AllAttachments`))))
      (for _array_element_2 (`local.AllAttachments`)
        (set `local.CurrentJig` _array_element_2)
        (bind _output_get (set `local.LocalInfo` (`/Game/_Game/JigSInventory/Jigsaw/Widgets/BP_Slot.GetJigDA` (`local.CurrentJig`))))
        (bind _local_actorclass (`/Game/_Game/JigSInventory/Jigsaw/Data/DataAsset/JigsawItem_DataAsset.Local_ActorClass` _output_get))
        (if (`KismetSystemLibrary.IsValidClass` _local_actorclass)
          (bind _returnvalue (`|SpawnActorFromClass` _local_actorclass (`KismetMathLibrary.MakeTransform` (`self.K2_GetActorLocation`)) "Undefined" "OverrideRootScale" null null))
          (`/Engine/EditorBlueprintResources/StandardMacros.IsValid` _returnvalue
            (:`Is Valid`
              (set `local.SpawnedItem` _returnvalue)
              (`KismetArrayLibrary.Array_Add` (`self.CurrentAttachments`) _returnvalue)
              (`/Game/_Game/JigSInventory/Jigsaw/Pickup/BP_AMainLocalAttachment.Jig_SetAttachmentInfo` _returnvalue (`/Game/_Game/JigSInventory/Jigsaw/Widgets/BP_Slot.GetUniqueID` (`local.CurrentJig`)) (`local.LocalInfo`))
              (set `local.ParentUID` (`/Game/_Game/JigSInventory/Jigsaw/Widgets/WBP_Container.GetSlotMotherUID` (`/Game/_Game/JigSInventory/Jigsaw/Widgets/BP_Slot.ContainerMother` (`local.CurrentJig`)) false false))
              (if (== (`local.ParentUID`) (`/Game/_Game/JigSInventory/Jigsaw/Widgets/BP_Slot.GetUniqueID` (`local.JigItem`)))
                (bind _comp (message `/Game/_Game/JigSInventory/Jigsaw/Pickup/BP_WeaponAttachments.Jig_GetPrimitiveComponent` (`local.SpawnedItem`)))
                (`SceneComponent.K2_AttachToComponent` _comp (`self.GetActiveComponent`) (`/Game/_Game/JigSInventory/Jigsaw/Data/DataAsset/JigsawItem_DataAsset.Local_AttachSocket` (`local.LocalInfo`)) "SnapToTarget" "SnapToTarget" "KeepWorld" true)
                (else
                  ;[0 0.2186 1] Ex: an laser sight on a handguard, things that are installed on other attachments instead of the weapon itself.
                  (for _array_element_3 (`self.CurrentAttachments`)
                    (bind _uid (message `/Game/_Game/JigSInventory/Jigsaw/Pickup/BP_WeaponAttachments.Jig_GetAttachmentInfo` _array_element_3))
                    (if (== _uid (`local.ParentUID`))
                      (`|ExecutionSequence`
                        (:`then_0`
                          (bind _comp_2 (message `/Game/_Game/JigSInventory/Jigsaw/Pickup/BP_WeaponAttachments.Jig_GetPrimitiveComponent` _array_element_3))
                          (bind _comp_3 (message `/Game/_Game/JigSInventory/Jigsaw/Pickup/BP_WeaponAttachments.Jig_GetPrimitiveComponent` (`local.SpawnedItem`)))
                          (`SceneComponent.K2_AttachToComponent` _comp_3 _comp_2 (`self.GetAttachSocketByInContainerIndex` (`local.LocalInfo`) (`/Game/_Game/JigSInventory/Jigsaw/Widgets/WBP_Container.GetContainerIndex` (`/Game/_Game/JigSInventory/Jigsaw/Widgets/BP_Slot.ContainerMother` (`local.CurrentJig`)))) "SnapToTarget" "SnapToTarget" "KeepWorld" true))
                        (:`then_1`
                          (break)))))))))))
      (for _array_element_4 (`self.CurrentAttachments`)
        (bind _comp_4 (message `/Game/_Game/JigSInventory/Jigsaw/Pickup/BP_WeaponAttachments.Jig_GetPrimitiveComponent` _array_element_4))
        (`PrimitiveComponent.SetLightingChannels` _comp_4 false true false)
        (`KismetArrayLibrary.Array_Append` (`SceneCaptureComponent.ShowOnlyActors` (`self.SceneCaptureComponent2D`)) (`self.CurrentAttachments`))))))

(fn `IsActionbar`
  (params (ItemRef :type "/Game/_Game/JigSInventory/Jigsaw/Widgets/BP_Slot Object Reference"))
  (returns (Result :type Boolean))
  (return (`/Game/_Game/JigSInventory/Jigsaw/Widgets/WBP_Container.IsActionbar` (`/Game/_Game/JigSInventory/Jigsaw/Widgets/BP_Slot.ContainerMother` ItemRef))))

(fn `IsLocked`
  (returns (`IsLocked?` :type Boolean))
  (return (`self.IsLocked?`)))

(fn `SetJigitem`
  (params (ItemRef :type "/Game/_Game/JigSInventory/Jigsaw/Widgets/BP_Slot Object Reference"))
  (returns (Found :type Boolean) (ShareRenderTargetWithSimilarItems :type Boolean))
  (locals (IsActionBarItem :type Boolean :default false))
  (bind _isactionbaritem (`local.IsActionBarItem`))
  ;[0.05208 0.05208 0.05208] Set the mesh to inspect
  (bind _output_get (set `self.ItemToInspect` ItemRef))
  (set `local.IsActionBarItem` (`self.IsActionbar` _output_get))
  (`|ExecutionSequence`
    (:`then_0`
      (bind _jigdataasset (`/Game/_Game/JigSInventory/Jigsaw/Widgets/BP_Slot.GetJigDA` _output_get))
      (if (`/Game/_Game/JigSInventory/Jigsaw/Data/DataAsset/JigsawItem_DataAsset.UseAsInventoryImage?` _jigdataasset)
        (`|ExecutionSequence`
          (:`then_0`
            (`StaticMeshComponent.SetStaticMesh` (`self.StaticMesh`) null)
            (`SkinnedMeshComponent.SetSkinnedAssetAndUpdate` (`self.SkeletalMesh`) null false)
            (bind (_actionbartransform_location _actionbartransform_rotation) (`KismetMathLibrary.BreakTransform` (`/Game/_Game/JigSInventory/Jigsaw/Data/DataAsset/JigsawItem_DataAsset.ActionbarTransform` _jigdataasset)))
            (bind (_inspecttransform_location _inspecttransform_rotation) (`KismetMathLibrary.BreakTransform` (`/Game/_Game/JigSInventory/Jigsaw/Data/DataAsset/JigsawItem_DataAsset.InspectTransform` _jigdataasset)))
            (`SceneComponent.K2_SetRelativeLocationAndRotation` (`self.SkeletalMesh`) (`KismetMathLibrary.SelectVector` _actionbartransform_location _inspecttransform_location _isactionbaritem) (`KismetMathLibrary.SelectRotator` _actionbartransform_rotation _inspecttransform_rotation _isactionbaritem) false true)
            (`SceneComponent.K2_SetRelativeLocationAndRotation` (`self.StaticMesh`) (`KismetMathLibrary.SelectVector` _actionbartransform_location _inspecttransform_location _isactionbaritem) (`KismetMathLibrary.SelectRotator` _actionbartransform_rotation _inspecttransform_rotation _isactionbaritem) false true))
          (:`then_1`
            (bind _skelmeshtoinspect (`/Game/_Game/JigSInventory/Jigsaw/Data/DataAsset/JigsawItem_DataAsset.SkelMeshToInspect` _jigdataasset))
            (`/Engine/EditorBlueprintResources/StandardMacros.IsValid` _skelmeshtoinspect
              (:`Is Valid`
                (`SkinnedMeshComponent.SetSkinnedAssetAndUpdate` (`self.SkeletalMesh`) _skelmeshtoinspect false))
              (:`Is Not Valid`
                (`StaticMeshComponent.SetStaticMesh` (`self.StaticMesh`) (`/Game/_Game/JigSInventory/Jigsaw/Data/DataAsset/JigsawItem_DataAsset.StaticMeshToInspect` _jigdataasset))))
            (bind _jigdataasset_2 (`/Game/_Game/JigSInventory/Jigsaw/Widgets/BP_Slot.GetJigDA` _output_get))
            (set `SceneCaptureComponent2D.FOVAngle` (`KismetMathLibrary.SelectFloat` (`/Game/_Game/JigSInventory/Jigsaw/Data/DataAsset/JigsawItem_DataAsset.ActionbarFOV` _jigdataasset_2) (`/Game/_Game/JigSInventory/Jigsaw/Data/DataAsset/JigsawItem_DataAsset.FOV` _jigdataasset_2) (`local.IsActionBarItem`)) (`self.SceneCaptureComponent2D`))
            (return true (`/Game/_Game/JigSInventory/Jigsaw/Data/DataAsset/JigsawItem_DataAsset.ShareSnapWithSimilarItems?` _jigdataasset))))
        (else
          (return false false))))
    (:`then_1`
      (return false false))))

(fn `SetJigitem_Custom`
  (params (ItemRef :type "/Game/_Game/JigSInventory/Jigsaw/Widgets/BP_Slot Object Reference") (Location :type "Vector Structure") (Rotation :type "Rotator Structure") (FOV :type "Float (double-precision)"))
  (returns (Found :type Boolean) (ShareRenderTargetWithSimilarItems :type Boolean))
  (locals (IsActionBarItem :type Boolean :default false))
  ;[0.05208 0.05208 0.05208] Set the mesh to inspect
  (bind _output_get (set `self.ItemToInspect` ItemRef))
  (`|ExecutionSequence`
    (:`then_0`
      (bind _jigdataasset (`/Game/_Game/JigSInventory/Jigsaw/Widgets/BP_Slot.GetJigDA` _output_get))
      (if (`/Game/_Game/JigSInventory/Jigsaw/Data/DataAsset/JigsawItem_DataAsset.UseAsInventoryImage?` _jigdataasset)
        (`|ExecutionSequence`
          (:`then_0`
            (`self.ClearAttachments`)
            (`StaticMeshComponent.SetStaticMesh` (`self.StaticMesh`) null)
            (`SkinnedMeshComponent.SetSkinnedAssetAndUpdate` (`self.SkeletalMesh`) null false)
            (`SceneComponent.K2_SetRelativeLocationAndRotation` (`self.SkeletalMesh`) (`local.Location`) (`local.Rotation`) false true)
            (`SceneComponent.K2_SetRelativeLocationAndRotation` (`self.StaticMesh`) (`local.Location`) (`local.Rotation`) false true))
          (:`then_1`
            (bind _skelmeshtoinspect (`/Game/_Game/JigSInventory/Jigsaw/Data/DataAsset/JigsawItem_DataAsset.SkelMeshToInspect` _jigdataasset))
            (`/Engine/EditorBlueprintResources/StandardMacros.IsValid` _skelmeshtoinspect
              (:`Is Valid`
                (`SkinnedMeshComponent.SetSkinnedAssetAndUpdate` (`self.SkeletalMesh`) _skelmeshtoinspect false))
              (:`Is Not Valid`
                (`StaticMeshComponent.SetStaticMesh` (`self.StaticMesh`) (`/Game/_Game/JigSInventory/Jigsaw/Data/DataAsset/JigsawItem_DataAsset.StaticMeshToInspect` _jigdataasset))))
            (set `SceneCaptureComponent2D.FOVAngle` (`local.FOV`) (`self.SceneCaptureComponent2D`))
            (return true (`/Game/_Game/JigSInventory/Jigsaw/Data/DataAsset/JigsawItem_DataAsset.ShareSnapWithSimilarItems?` _jigdataasset))))
        (else
          (return false false))))
    (:`then_1`
      (return false false))))

(fn `SetLocked`
  (params (`IsLocked?` :type Boolean))
  (set `self.IsLocked?` `IsLocked?`))

(fn `UpdateSnap`
  (params (ItemRef :type "/Game/_Game/JigSInventory/Jigsaw/Widgets/BP_Slot Object Reference") (TextureTarget :type "TextureRenderTarget2D Object Reference"))
  (returns (Output_Get :type "TextureRenderTarget2D Object Reference"))
  (bind _scenecapturecomponent2d (`self.SceneCaptureComponent2D`))
  (`self.SetJigitem` ItemRef)
  (bind _output_get (set `SceneCaptureComponent2D.TextureTarget` TextureTarget _scenecapturecomponent2d))
  (`SceneCaptureComponent2D.CaptureScene` _scenecapturecomponent2d)
  (set `SceneCaptureComponent2D.TextureTarget` null _scenecapturecomponent2d)
  (return _output_get))

(fn `UserConstructionScript`
  (set `SceneCaptureComponent.ShowOnlyActors` (`|MakeArray` self :!type "Actor Object Reference") (`self.SceneCaptureComponent2D`)))