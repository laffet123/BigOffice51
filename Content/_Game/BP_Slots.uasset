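; BP_Slots is an Actor that sketches slot-grid occupancy, apparently for placing items that span several columns and rows.
; CalVector truncates a start vector to a column and row, adds the given extents, and loops over that rectangle to flag each slot as not empty.
; The GetSlot_FromIndex lookup and SetIsEmpty setter it relies on are empty stubs, and the default events do nothing.
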(fn `Cal_Vector`
  (params (FirstVector :type "Vector2D Structure") (Columns :type Integer) (Rows :type Integer))
  (locals (FirstCol :type Integer :default 0) (FirstRow :type Integer :default 0) (LastCol :type Integer) (LastRow :type Integer))
  (bind (_x _y) (`KismetMathLibrary.BreakVector2D` (`local.FirstVector`)))
  (`|ExecutionSequence`
    (:`then_0`
      (set `local.FirstCol` (`KismetMathLibrary.FTrunc` _x))
      (set `local.FirstRow` (`KismetMathLibrary.FTrunc` _y))
      (set `local.LastCol` (+ (`local.FirstCol`) (`local.Columns`)))
      (set `local.LastRow` (+ (`local.FirstRow`) (`local.Rows`))))
    (:`then_1`
      (for _index (range (`local.FirstCol`) (+ (`local.LastCol`) 1))
        (for _index_2 (range (`local.FirstRow`) (+ (`local.LastRow`) 1))
          (`self.SetIsEmpty` (`self.GetSlot_FromIndex` _index _index_2) false))))))

(fn `SetIsEmpty`
  (params (`IsEmpty?` :type Boolean)))

(fn `UserConstructionScript`)