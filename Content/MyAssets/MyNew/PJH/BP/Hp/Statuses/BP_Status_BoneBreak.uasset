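; Bone-break status effect in the HP system that slows the afflicted character while active.
; On initialization it casts the HP system's owner to BP_CharRoot and lowers the movement component's max walk speed.
; On removal it sets a hard-coded normal speed instead of restoring the previous value.
; The per-tick effect only calls the parent implementation.
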(event `self.SecEffect`
  (params (tickTime :type "Float (double-precision)"))
  (`parent.SecEffect` tickTime))

(event `self.Initialize`
  (params (Input_Wbp_HpOverlayRef :type "/Game/MyAssets/MyNew/PJH/BP/Hp/Widget/WBP_HpOverlay Object Reference"))
  (`parent.Initialize` Input_Wbp_HpOverlayRef)
  (set `CharacterMovementComponent.MaxWalkSpeed` 100.0 (`Character.CharacterMovement` (cast `/Game/MyAssets/MyNew/PJH/BP/CharRoot/BP_CharRoot` (`ActorComponent.GetOwner` (`self.Owner_HpSystem`)) :!pure true))))

(event `self.OnStatusRemoved`
  (`parent.OnStatusRemoved`)
  (set `CharacterMovementComponent.MaxWalkSpeed` 400.0 (`Character.CharacterMovement` (cast `/Game/MyAssets/MyNew/PJH/BP/CharRoot/BP_CharRoot` (`ActorComponent.GetOwner` (`self.Owner_HpSystem`)) :!pure true))))