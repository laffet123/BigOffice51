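; BP_AMainLocalAttachment is an attachment actor for the Jigsaw inventory system, built around a static mesh.
; It stores an attachment UID and info through interface-style Jig functions, exposes the mesh, and reports its "ADS" socket location for aiming.
; The weapon-related functions for chambering, reloading, magazines, equip montage and nested attachments are stubs that return false or empty results.
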(fn `Jig_AttachmentInstalled`
  (params (MainUID :type "Guid Structure") (Attachments :type "Array of /Game/JigSInventory/Jigsaw/Data/S_RepAttachmentInfo Structure (by ref)"))
  (returns (Result :type Boolean) (AttachmentType :type "/Game/JigSInventory/Jigsaw/Data/AttachmentType Enum"))
  (return false "NewEnumerator0"))

(fn `Jig_AttachmentRemoved`
  (params (Attachments :type "Array of /Game/JigSInventory/Jigsaw/Data/S_RepAttachmentInfo Structure (by ref)"))
  (returns (Result :type Boolean) (AttachmentType :type "/Game/JigSInventory/Jigsaw/Data/AttachmentType Enum"))
  (return false "NewEnumerator0"))

(fn `Jig_CanChamberWeapon`
  (params (MPComp :type "/Game/JigSInventory/Jigsaw/Components/BP_Multiplayer Object Reference") (PlayerSlots :type "/Game/JigSInventory/Jigsaw/Data/PlayerSlots Enum" :default "NewEnumerator0"))
  (returns (Result :type Boolean))
  (return false))

(fn `Jig_CheckCanReload`
  (params (MPComp :type "/Game/JigSInventory/Jigsaw/Components/BP_Multiplayer Object Reference") (PlayerSlots :type "/Game/JigSInventory/Jigsaw/Data/PlayerSlots Enum" :default "NewEnumerator0"))
  (returns (Result :type Boolean) (ContainerMag :type "/Game/JigSInventory/Jigsaw/Widgets/WBP_Container Object Reference") (ReloadMontage :type "AnimMontage Object Reference") (HasInternalMag :type Boolean) (`CanChamber?` :type Boolean) (ReloadWith :type "/Game/JigSInventory/Jigsaw/Widgets/BP_Slot Object Reference") (LoopReloadAnim :type "AnimMontage Object Reference"))
  (return false null null false false null null))

(fn `Jig_ExecuteChamberWeapon`
  (params (MPComp :type "/Game/JigSInventory/Jigsaw/Components/BP_Multiplayer Object Reference") (PlayerSlots :type "/Game/JigSInventory/Jigsaw/Data/PlayerSlots Enum" :default "NewEnumerator0"))
  (returns (Result :type Boolean) (ChamberMontage :type "AnimMontage Object Reference"))
  (return false null))

(fn `Jig_GetADSSocketLocation`
  (returns (SocketLoc :type "Vector Structure") (SocketFound :type Boolean))
  (bind _staticmesh (`self.StaticMesh`))
  (return (`SceneComponent.GetSocketLocation` _staticmesh "ADS") (`SceneComponent.DoesSocketExist` _staticmesh "ADS")))

(fn `Jig_GetAttachmentByType`
  (params (Type :type "/Game/JigSInventory/Jigsaw/Data/AttachmentType Enum" :default "NewEnumerator9"))
  (returns (Attachment :type "/Game/JigSInventory/Jigsaw/Pickup/BP_AMainLocalAttachment Object Reference") (Found :type Boolean))
  (return null false))

(fn `Jig_GetAttachmentInfo`
  (returns (UID :type "Guid Structure") (AttachmentInfo :type "/Game/JigSInventory/Jigsaw/Data/DataAsset/JigsawItem_DataAsset Object Reference"))
  (return (`self.AttachmentUID`) (`self.Attachment Info`)))

(fn `Jig_GetEquipMontage`
  (params (`CanChamber?` :type Boolean))
  (returns (EquipMontage :type "AnimMontage Object Reference"))
  (return null))

(fn `Jig_GetPendingMag`
  (params (`FindMagIfNoPending?` :type Boolean))
  (returns (MagRef :type "/Game/JigSInventory/Jigsaw/Pickup/BP_AMainLocalAttachment Object Reference"))
  (return null))

(fn `Jig_GetPrimitiveComponent`
  (returns (Comp :type "PrimitiveComponent Object Reference"))
  (return (`self.StaticMesh`)))

(fn `Jig_SetAttachmentInfo`
  (params (UID :type "Guid Structure") (AttachmentInfo :type "/Game/JigSInventory/Jigsaw/Data/DataAsset/JigsawItem_DataAsset Object Reference"))
  (returns (Result :type Boolean))
  (set `self.AttachmentUID` UID)
  (set `self.Attachment Info` AttachmentInfo)
  (return true))

(fn `Jig_SetPendindMag`
  (params (MagRef :type "/Game/JigSInventory/Jigsaw/Pickup/BP_AMainLocalAttachment Object Reference"))
  (returns (Result :type Boolean))
  (return false))

(fn `Jig_StartReloading`
  (params (MPCom :type "/Game/JigSInventory/Jigsaw/Components/BP_Multiplayer Object Reference") (MagContainer :type "/Game/JigSInventory/Jigsaw/Widgets/WBP_Container Object Reference"))
  (returns (Result :type Boolean))
  (return false))

(fn `UserConstructionScript`)