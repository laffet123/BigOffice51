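; Inventory item inspector actor that renders an item's static or skeletal mesh into a render target through a show-only scene capture.
; Mesh, transform and zoom limits come from the item's data asset; a spring arm handles rotation and capture FOV handles zoom.
; Equipped attachments spawn as local actors matched by UID, snapped to sockets on the item or parent attachment.
; While the capture component is inactive, changes like zoom trigger single-frame captures.
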(event `self.ReceiveBeginPlay`
  ;[0.02604 0.02604 0.02604] Begin play
  (set `SceneCaptureComponent2D.FOVAngle` (`self.InitialFOV`) (`self.SceneCaptureComponent2D`))
  (set `SceneCaptureComponent.MaxViewDistanceOverride` 1000.0 (`self.SceneCaptureComponent2D`)))

(event `self.ReceiveEndPlay`
  (params (EndPlayReason :type "EEndPlayReason Enum" :default "Destroyed"))
  (bind _currentattachments (`self.CurrentAttachments`))
  ;[0.005208 0.005208 0.005208] End play
  (set `/Game/JigSInventory/Jigsaw/Widgets/JSI_Slot.InspectorWidget` null (`self.ItemToInspect`))
  (`KismetRenderingLibrary.ReleaseRenderTarget2D` (`self.RenderT`))
  (bind (_arrayindex _arrayelement) (`/Engine/EditorBlueprintResources/StandardMacros.ReverseForEachLoop` _currentattachments)
    (:`LoopBody`
      (`self.K2_DestroyActor` _arrayelement))
    (:`Completed`
      (`KismetArrayLibrary.Array_Clear` _currentattachments))))

(fn `Capture One Frame`
  (if (not (`ActorComponent.IsActive` (`self.SceneCaptureComponent2D`)))
    (`SceneCaptureComponent2D.CaptureScene` (`self.SceneCaptureComponent2D`))))

(fn `ClearAttachments`
  (bind _currentattachments (`self.CurrentAttachments`))
  (bind _showonlyactors (`SceneCaptureComponent.ShowOnlyActors` (`self.SceneCaptureComponent2D`)))
  (`KismetArrayLibrary.Array_Clear` _showonlyactors)
  (`KismetArrayLibrary.Array_Add` _showonlyactors self)
  (bind (_arrayindex _arrayelement) (`/Engine/EditorBlueprintResources/StandardMacros.ReverseForEachLoop` _currentattachments)
    (:`LoopBody`
      (`self.K2_DestroyActor` _arrayelement))
    (:`Completed`
      (`KismetArrayLibrary.Array_Clear` _currentattachments))))

(fn `FindLocalAttachmentByUID`
  (params (UID :type "Guid Structure"))
  (returns (Attachment :type "/Game/JigSInventory/Jigsaw/Pickup/BP_AMainLocalAttachment Object Reference"))
  (for _array_element (`self.CurrentAttachments`)
    (bind _uid (message `/Game/JigSInventory/Jigsaw/Pickup/BP_WeaponAttachments.Jig_GetAttachmentInfo` _array_element))
    (if (== _uid (`local.UID`))
      (return _array_element)))
  (return null))

(fn `GetActiveComponent`
  (returns (Comp :type "SceneComponent Object Reference"))
  (`/Engine/EditorBlueprintResources/StandardMacros.IsValid` (`StaticMeshComponent.StaticMesh` (`self.StaticMesh`))
    (:`Is Valid`
      (return (`self.StaticMesh`)))
    (:`Is Not Valid`
      (return (`self.SkeletalMesh`)))))

(fn `GetAttachSocketByInContainerIndex`
  (params (Info :type "/Game/JigSInventory/Jigsaw/Data/DataAsset/JigsawItem_DataAsset Object Reference") (InContainerIndex :type Integer))
  (returns (Socket :type Name))
  ;[1 1 1] In container index: Take a handguard for example, a laser sight could be installed to the left or the right side, so we determine the socket based on InContainerIndex.
  ; This depends on how you setup your special container.
  (`|ExecutionSequence`
    (:`then_0`
      (for _array_element (`/Game/JigSInventory/Jigsaw/Data/DataAsset/JigsawItem_DataAsset.Local_AttachToSocketByContainerIndex` Info)
        (bind (_index _socketname) (break `/Game/JigSInventory/Jigsaw/Pickup/S_LocalAttContainerIndexSocket` _array_element))
        (if (== _index (`local.InContainerIndex`))
          (return _socketname))))
    (:`then_1`
      (return (`/Game/JigSInventory/Jigsaw/Data/DataAsset/JigsawItem_DataAsset.Local_AttachSocket` Info)))))

(fn `GetInitValues`
  (returns (ReturnValue :type "Transform Structure") (FOVAngle :type "Float (double-precision)"))
  (bind _skeletalmesh (`self.SkeletalMesh`))
  (return (`SceneComponent.GetRelativeTransform` (select `bool` (`KismetSystemLibrary.IsValid` (`SkinnedMeshComponent.SkeletalMesh` _skeletalmesh)) :`false` (`self.StaticMesh`) :`true` _skeletalmesh :!type "SceneComponent Object Reference")) (`SceneCaptureComponent2D.FOVAngle` (`self.SceneCaptureComponent2D`))))

(fn `GetRenderTarget`
  (returns (RenderT :type "TextureRenderTarget2D Object Reference"))
  (return (`self.RenderT`)))

(fn `InstallAttachments`
  (params (JigItem :type "/Game/JigSInventory/Jigsaw/Widgets/JSI_Slot Object Reference"))
  (locals (AllAttachments :type "Array of /Game/JigSInventory/Jigsaw/Widgets/JSI_Slot Object Reference") (CurrentJig :type "/Game/JigSInventory/Jigsaw/Widgets/JSI_Slot Object Reference") (SpawnedItem :type "/Game/JigSInventory/Jigsaw/Pickup/BP_AMainLocalAttachment Object Reference") (LocalInfo :type "/Game/JigSInventory/Jigsaw/Data/DataAsset/JigsawItem_DataAsset Object Reference") (ParentUID :type "Guid Structure") (AllJigUIDs :type "Array of Guid Structure"))
  (bind _containerref (`/Game/JigSInventory/Jigsaw/Widgets/JSI_Slot.GetContainerOneRef` JigItem))
  (bind _spawneditem (`local.SpawnedItem`))
  (bind _currentattachments (`self.CurrentAttachments`))
  (bind _spawneditem_2 (`local.SpawnedItem`))
  (bind _spawneditem_3 (`local.SpawnedItem`))
  (`KismetArrayLibrary.Array_Clear` (`local.AllAttachments`))
  (`/Engine/EditorBlueprintResources/StandardMacros.IsValid` _containerref
    (:`Is Valid`
      (bind _containers (message `/Game/JigSInventory/Jigsaw/Widgets/SpecialContainers/JSISpecialWidgetInterface.GetListOfContainers` _containerref))
      (for _array_element _containers
        (if (`/Game/JigSInventory/Jigsaw/Widgets/JSIContainer.IsEquipTo?` _array_element)
          (`/Game/JigSInventory/Jigsaw/Widgets/JSIContainer.Deep_GettAllItems` _array_element (`local.AllAttachments`))))
      (for _array_element_2 (`local.AllAttachments`)
        (bind _output_get (set `local.CurrentJig` _array_element_2))
        (bind _uniqueserverid (`/Game/JigSInventory/Jigsaw/Widgets/JSI_Slot.GetUniqueID` _output_get))
        (`KismetArrayLibrary.Array_Add` (`local.AllJigUIDs`) _uniqueserverid)
        (bind _attachment (`self.FindLocalAttachmentByUID` _uniqueserverid))
        (bind _output_get_2 (set `local.SpawnedItem` _attachment))
        (bind (_uid _attachmentinfo) (message `/Game/JigSInventory/Jigsaw/Pickup/BP_WeaponAttachments.Jig_GetAttachmentInfo` _output_get_2))
        (set `local.LocalInfo` _attachmentinfo)
        (`/Engine/EditorBlueprintResources/StandardMacros.IsValid` _output_get_2
          (:`Is Valid`
            (set `local.ParentUID` (`/Game/JigSInventory/Jigsaw/Widgets/JSIContainer.GetSlotMotherUID` (`/Game/JigSInventory/Jigsaw/Widgets/JSI_Slot.ContainerMother` (`local.CurrentJig`)) false false) :!label _label)
            (if (== (`local.ParentUID`) (`/Game/JigSInventory/Jigsaw/Widgets/JSI_Slot.GetUniqueID` (`local.JigItem`)))
              (message `/Game/JigSInventory/Jigsaw/Pickup/BP_WeaponAttachments.Jig_GetPrimitiveComponent` _spawneditem_3)
              (`SceneComponent.K2_AttachToComponent` (`Actor.RootComponent` _spawneditem_3) (`self.GetActiveComponent`) (`/Game/JigSInventory/Jigsaw/Data/DataAsset/JigsawItem_DataAsset.Local_AttachSocket` (`local.LocalInfo`)) "SnapToTarget" "SnapToTarget" "KeepWorld" true)
              (else
                ;[0 0.2186 1] Ex: an laser sight on a handguard, things that are installed on other attachments instead of the weapon itself.
                (bind _attachment_2 (`self.FindLocalAttachmentByUID` (`local.ParentUID`)))
                (`/Engine/EditorBlueprintResources/StandardMacros.IsValid` _attachment_2
                  (:`Is Valid`
                    (bind _comp (message `/Game/JigSInventory/Jigsaw/Pickup/BP_WeaponAttachments.Jig_GetPrimitiveComponent` _attachment_2))
                    (message `/Game/JigSInventory/Jigsaw/Pickup/BP_WeaponAttachments.Jig_GetPrimitiveComponent` _spawneditem_2)
                    (`SceneComponent.K2_AttachToComponent` (`Actor.RootComponent` _spawneditem_2) _comp (`self.GetAttachSocketByInContainerIndex` (`local.LocalInfo`) (`/Game/JigSInventory/Jigsaw/Widgets/JSIContainer.GetContainerIndex` (`/Game/JigSInventory/Jigsaw/Widgets/JSI_Slot.ContainerMother` (`local.CurrentJig`)))) "SnapToTarget" "SnapToTarget" "KeepWorld" true))))))
          (:`Is Not Valid`
            (set `local.LocalInfo` (`/Game/JigSInventory/Jigsaw/Widgets/JSI_Slot.GetJigDA` (`local.CurrentJig`)))
            (bind _returnvalue (`|SpawnActorFromClass` (`/Game/JigSInventory/Jigsaw/Data/DataAsset/JigsawItem_DataAsset.Local_ActorClass` (`/Game/JigSInventory/Jigsaw/Widgets/JSI_Slot.GetJigDA` (`local.CurrentJig`))) (`KismetMathLibrary.MakeTransform` (`self.K2_GetActorLocation`)) "Undefined" "OverrideRootScale" null null))
            (bind _output_get_3 (set `local.SpawnedItem` _returnvalue))
            (`/Engine/EditorBlueprintResources/StandardMacros.IsValid` _output_get_3
              (:`Is Valid`
                (`KismetArrayLibrary.Array_Add` (`self.CurrentAttachments`) _spawneditem)
                (`/Game/JigSInventory/Jigsaw/Pickup/BP_AMainLocalAttachment.Jig_SetAttachmentInfo` _spawneditem (`/Game/JigSInventory/Jigsaw/Widgets/JSI_Slot.GetUniqueID` (`local.CurrentJig`)) (`/Game/JigSInventory/Jigsaw/Widgets/JSI_Slot.GetJigDA` (`local.CurrentJig`)))
                (`|ExecutionSequence`
                  (:`then_0`
                    (bind _comp_2 (message `/Game/JigSInventory/Jigsaw/Pickup/BP_WeaponAttachments.Jig_GetPrimitiveComponent` _spawneditem))
                    (`PrimitiveComponent.SetLightingChannels` _comp_2 false true false)
                    (`KismetArrayLibrary.Array_Add` (`SceneCaptureComponent.ShowOnlyActors` (`self.SceneCaptureComponent2D`)) _spawneditem))
                  (:`then_1`
                    (goto _label))))))))
      ;[0.04688 0.04688 0.04688] Destroy non existing attachments
      (bind (_arrayindex _arrayelement) (`/Engine/EditorBlueprintResources/StandardMacros.ReverseForEachLoop` _currentattachments)
        (:`LoopBody`
          (bind _uid_2 (message `/Game/JigSInventory/Jigsaw/Pickup/BP_WeaponAttachments.Jig_GetAttachmentInfo` _arrayelement))
          (if (not (`KismetArrayLibrary.Array_Contains` (`local.AllJigUIDs`) _uid_2))
            (`KismetArrayLibrary.Array_RemoveItem` (`SceneCaptureComponent.ShowOnlyActors` (`self.SceneCaptureComponent2D`)) _arrayelement)
            (`self.K2_DestroyActor` _arrayelement)
            (`KismetArrayLibrary.Array_Remove` _currentattachments _arrayindex)))))))

(fn `OnZoomIn`
  (bind _scenecapturecomponent2d (`self.SceneCaptureComponent2D`))
  (set `SceneCaptureComponent2D.FOVAngle` (`KismetMathLibrary.FClamp` (+ (`SceneCaptureComponent2D.FOVAngle` _scenecapturecomponent2d) -5.0) (`self.MaxZoomInFOV`) (`self.MaxZoomOutFOV`)) _scenecapturecomponent2d)
  (if (not (`ActorComponent.IsActive` _scenecapturecomponent2d))
    (`self.Capture One Frame`)))

(fn `OnZoomOut`
  (bind _scenecapturecomponent2d (`self.SceneCaptureComponent2D`))
  (set `SceneCaptureComponent2D.FOVAngle` (`KismetMathLibrary.FClamp` (+ (`SceneCaptureComponent2D.FOVAngle` _scenecapturecomponent2d) 5.0) (`self.MaxZoomInFOV`) (`self.MaxZoomOutFOV`)) _scenecapturecomponent2d)
  (if (not (`ActorComponent.IsActive` _scenecapturecomponent2d))
    (`self.Capture One Frame`)))

(fn `SetCaptorActiveState`
  (params (IsActive :type Boolean))
  (`ActorComponent.SetActive` (`self.SceneCaptureComponent2D`) IsActive false))

(fn `SetItemToInspect`
  (params (ItemRef :type "/Game/JigSInventory/Jigsaw/Widgets/JSI_Slot Object Reference"))
  (bind _staticmesh (`self.StaticMesh`))
  (bind _skeletalmesh (`self.SkeletalMesh`))
  (`|ExecutionSequence`
    (:`then_0`
      ;[1 1 1] Create the render target
      (bind _returnvalue (`KismetRenderingLibrary.CreateRenderTarget2D` 512 512))
      (bind _output_get (set `SceneCaptureComponent2D.TextureTarget` _returnvalue (`self.SceneCaptureComponent2D`)))
      (set `self.RenderT` _output_get))
    (:`then_1`
      ;[0.05208 0.05208 0.05208] Set the mesh to inspect
      (bind _output_get_2 (set `self.ItemToInspect` ItemRef))
      (`|ExecutionSequence`
        (:`then_0`
          (`|ExecutionSequence`
            (:`then_0`
              (`StaticMeshComponent.SetStaticMesh` (`self.StaticMesh`) null)
              (`SkinnedMeshComponent.SetSkinnedAssetAndUpdate` (`self.SkeletalMesh`) null false))
            (:`then_1`
              (bind _jigdataasset (`/Game/JigSInventory/Jigsaw/Widgets/JSI_Slot.GetJigDA` _output_get_2))
              (bind _skelmeshtoinspect (`/Game/JigSInventory/Jigsaw/Data/DataAsset/JigsawItem_DataAsset.SkelMeshToInspect` _jigdataasset))
              (`/Engine/EditorBlueprintResources/StandardMacros.IsValid` _skelmeshtoinspect
                (:`Is Valid`
                  (`SkinnedMeshComponent.SetSkinnedAssetAndUpdate` _skeletalmesh _skelmeshtoinspect false)
                  (bind (_inspecttransform_location _inspecttransform_rotation) (`KismetMathLibrary.BreakTransform` (`/Game/JigSInventory/Jigsaw/Data/DataAsset/JigsawItem_DataAsset.InspectTransform` _jigdataasset)))
                  (`SceneComponent.K2_SetRelativeLocationAndRotation` _skeletalmesh _inspecttransform_location _inspecttransform_rotation false true))
                (:`Is Not Valid`
                  (`StaticMeshComponent.SetStaticMesh` _staticmesh (`/Game/JigSInventory/Jigsaw/Data/DataAsset/JigsawItem_DataAsset.StaticMeshToInspect` _jigdataasset))
                  (bind _jigdataasset_2 (`/Game/JigSInventory/Jigsaw/Widgets/JSI_Slot.GetJigDA` _output_get_2))
                  (bind (_inspecttransform_location_2 _inspecttransform_rotation_2) (`KismetMathLibrary.BreakTransform` (`/Game/JigSInventory/Jigsaw/Data/DataAsset/JigsawItem_DataAsset.InspectTransform` _jigdataasset_2)))
                  (`SceneComponent.K2_SetRelativeLocationAndRotation` _staticmesh _inspecttransform_location_2 _inspecttransform_rotation_2 false true)))
              (set `self.MaxZoomInFOV` (`/Game/JigSInventory/Jigsaw/Data/DataAsset/JigsawItem_DataAsset.MaxZoomIn` _jigdataasset_2))
              (set `self.MaxZoomOutFOV` (`/Game/JigSInventory/Jigsaw/Data/DataAsset/JigsawItem_DataAsset.MaxZoomOut` _jigdataasset_2))
              (set `SceneCaptureComponent2D.FOVAngle` (`/Game/JigSInventory/Jigsaw/Data/DataAsset/JigsawItem_DataAsset.FOV` _jigdataasset_2) (`self.SceneCaptureComponent2D`)))))
        (:`then_1`
          (`SceneCaptureComponent2D.CaptureScene` (`self.SceneCaptureComponent2D`)))))))

(fn `SetMeshRotation`
  (params (XYRot :type "Vector2D Structure"))
  (`SceneComponent.K2_AddLocalRotation` (`self.SpringArm`) (`KismetMathLibrary.MakeRotator` 0.0 XYRot_Y (* XYRot_X -1.0)) false false))

(fn `UpdateLocAndRot`
  (params (NewLocation :type "Vector Structure") (NewRotation :type "Rotator Structure") (FOVAngle :type "Float (double-precision)"))
  (`SceneComponent.K2_SetRelativeLocationAndRotation` (`self.StaticMesh`) NewLocation NewRotation false true)
  (`SceneComponent.K2_SetRelativeLocationAndRotation` (`self.SkeletalMesh`) NewLocation NewRotation false true)
  (set `SceneCaptureComponent2D.FOVAngle` FOVAngle (`self.SceneCaptureComponent2D`))
  (`self.Capture One Frame`))

(fn `UserConstructionScript`
  (set `SceneCaptureComponent.ShowOnlyActors` (`|MakeArray` self :!type "Actor Object Reference") (`self.SceneCaptureComponent2D`)))