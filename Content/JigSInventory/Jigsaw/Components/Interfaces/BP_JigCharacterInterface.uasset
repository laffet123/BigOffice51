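; Blueprint interface for the player character in the Jigsaw inventory system, declaring the calls it answers for inventory and interaction.
; It covers adding UI widgets, pickup interaction, out-of-range interact actors, special container attachment updates and trace ignore lists.
; It also handles server and client data requests, saved-data loading, weapon ammo checks and animation state queries such as active slot, lean, ADS and crouch.
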(fn `AddJigWidgetToContent`
  (params (WidgetRef :type "UserWidget Object Reference") (ContentName :type Text))
  (returns (Result :type Boolean))
  (return false))

(fn `GetAnimationInfo`
  (returns (ActiveSlot :type "/Game/JigSInventory/Jigsaw/Data/PlayerSlots Enum") (Leaning :type "Float (double-precision)") (Ads :type Boolean) (Crouched :type Boolean) (`IsFirstPerson?` :type Boolean) (WeaponID :type Name))
  (return "NewEnumerator0" 0.0 false false false "None"))

(fn `GetTraceActorsToIgnore`
  (returns (Actors :type "Array of Actor Object Reference"))
  (return))

(fn `JigCheckWeaponAmmoCount`
  (returns (Result :type Boolean))
  (return false))

(fn `OnClientDataRequested`
  (params (ActionbarUIDs :type "Array of Guid Structure"))
  (returns (Result :type Boolean))
  (return false))

(fn `OnInteractActorOverDistance`
  (params (ActorRef :type "Actor Object Reference"))
  (returns (Result :type Boolean))
  (return false))

(fn `OnLoadSavedDataRequested`
  (params (PlayerLocation :type "Vector Structure") (MapName :type String))
  (returns (Result :type Boolean))
  (return false))

(fn `OnPickupInteractExecuted`
  (params (PickupRef :type "Actor Object Reference"))
  (returns (Result :type Boolean))
  (return false))

(fn `OnSpecialContainerattachmentUpdated`
  (params (ItemRef :type "/Game/JigSInventory/Jigsaw/Widgets/JSI_Slot Object Reference"))
  (returns (Result :type Boolean))
  (return false))

(fn `RequestServerData`
  (params (TargetComp :type "/Game/JigSInventory/Jigsaw/Components/BP_JigMultiplayer Object Reference"))
  (returns (Result :type Boolean))
  (return false))